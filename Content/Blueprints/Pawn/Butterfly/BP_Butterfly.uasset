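; Origami butterfly that waits along a placed path and flies on to the next point each time BP_Hero enters its approach sphere, with an attached flight sound event.
; A timeline lerps it straight between consecutive spline points over a set duration, facing the target and flapping, then restores its initial rotation and idle animation.
; A move request at path index 1 also applies a gameplay effect to the player through GAS.
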(event OnComponentBeginOverlap(SphereAceApproaches)
  (params (OverlappedComponent :type Primitive%20Component%20Object%20Reference) (OtherActor :type Actor%20Object%20Reference) (OtherComp :type Primitive%20Component%20Object%20Reference) (OtherBodyIndex :type Integer) (bFromSweep :type Boolean) (SweepResult :type Hit%20Result%20Structure%20%28by%20ref%29))
  (if (== (Utilities|GetClass OtherActor) "/Game/Blueprints/Character/Hero/BP_Hero.BP_Hero_C")
    (CallFunction|MovetoNextLocation)
    (Class|FMODBlueprintStatics|PlayEventAttached "/Game/FMOD/Events/SFX/NPC/Butterfly/ButterflyFly.ButterflyFly" (Variables|Transformation|GetRootComponent) "None" "0, 0, 0" "KeepRelativeOffset")))

(event Custom|Move%20To%20Next%20Location
  (bind _pathtofollow (Variables|Default|GetPathToFollow))
  (bind _pathlocation (Variables|Default|GetPathLocation))
  (bind _pathlocation_2 (Variables|Default|GetPathLocation))
  (bind _pathindex (Variables|Default|GetPathIndex))
  (bind _returnvalue (+ _pathindex 1))
  (bind _spline (Variables|/Game/Blueprints/Pawn/Butterfly/BP_ButterflyPath.BP_ButterflyPath_C|GetSpline _pathtofollow))
  (bind _returnvalue_2 (Spline|GetSplinePointAt _spline _pathindex "Local"))
  (bind _returnvalue_3 (Spline|GetSplinePointAt _spline _returnvalue "Local"))
  (bind _returnvalue_4 (+ _pathlocation (.position _returnvalue_2)))
  (bind _returnvalue_5 (+ (.position _returnvalue_3) _pathlocation_2))
  (if (== (Variables|Default|GetPathIndex) 1)
    (GameplayEffects|ApplyGameplayEffectToSelf :self (Ability|GetAbilitySystemComponent (Game|GetPlayerCharacter 0)) :GameplayEffectClass (Variables|Default|GetGameplay%20Effect%20First%20Move)))
  (if (and (> (Spline|GetNumberOfSplinePoints (Variables|/Game/Blueprints/Pawn/Butterfly/BP_ButterflyPath.BP_ButterflyPath_C|GetSpline (Variables|Default|GetPathToFollow))) (+ (Variables|Default|GetPathIndex) 1)) (not (Variables|Default|GetIsMoving)))
    (Components|Animation|PlayAnimation (Variables|Default|GetSM_Origami_Butterfly) "/Game/Assets/Character/OrigamiButterfly/Animations/AS_OrigamiButterfly_Flapping.AS_OrigamiButterfly_Flapping" true)
    (Variables|Default|SetIsMoving true)
    (Components|Timeline|SetPlayRate (Variables|Default|GetMove%20Object%20T) (/ 1.0 (Variables|Default|GetTime%20To%20Complete%20%28In%20Seconds%29)))
    (Transformation|SetActorRotation (Math|Rotator|FindLookatRotation _returnvalue_4 _returnvalue_5))
    (bind _move_track (Timeline|Move%20Object%20T PlayFromStart)
      (:Update
        (Transformation|SetActorLocation (Math|Vector|Lerp(Vector) _returnvalue_4 _returnvalue_5 _move_track) false false))
      (:Finished
        (Math|Integer|IncrementInt (Variables|Default|GetPathIndex)
          (:%20%20
            (Variables|Default|SetIsMoving false)
            (Transformation|SetActorRotation (Variables|Default|GetInitialRotation))
            (Components|Animation|PlayAnimation (Variables|Default|GetSM_Origami_Butterfly) "/Game/Assets/Character/OrigamiButterfly/Animations/AS_OrigamiButterfly_Idle.AS_OrigamiButterfly_Idle" true)))))))

(event EventBeginPlay
  (bind _pathtofollow (Variables|Default|GetPathToFollow))
  (Variables|Default|SetPathLocation (Transformation|GetActorLocation _pathtofollow))
  (Transformation|SetActorLocation (+ (.position (Spline|GetSplinePointAt (Variables|/Game/Blueprints/Pawn/Butterfly/BP_ButterflyPath.BP_ButterflyPath_C|GetSpline _pathtofollow) 0 "Local")) (Variables|Default|GetPathLocation)) false true)
  (Variables|Default|SetInitialRotation (Transformation|GetActorRotation))
  (Components|Animation|PlayAnimation (Variables|Default|GetSM_Origami_Butterfly) "/Game/Assets/Character/OrigamiButterfly/Animations/AS_OrigamiButterfly_Idle.AS_OrigamiButterfly_Idle" true))

(fn ConstructionScript)