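; BP_Mark2 is a mark projectile that activates objects it touches which match the Activable.Mark gameplay tag.
; On BeginPlay it homes on HomingTarget's root component, or without a valid target it flies unguided with a short lifespan.
; A sphere overlap sends the activate message to matching actors and destroys the projectile, which is also destroyed on reaching its homing target.
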(event OnComponentBeginOverlap(Sphere)
  (params (OverlappedComponent :type Primitive%20Component%20Object%20Reference) (OtherActor :type Actor%20Object%20Reference) (OtherComp :type Primitive%20Component%20Object%20Reference) (OtherBodyIndex :type Integer) (bFromSweep :type Boolean) (SweepResult :type Hit%20Result%20Structure%20%28by%20ref%29))
  (bind _returnvalue (GameplayTags|HasMatchingGameplayTag(Message) OtherActor "(TagName=\"Activable.Mark\")"))
  (if _returnvalue
    (Class|KrakenActivableObject|Activate(Message) OtherActor)
    (Actor|DestroyActor :!label _label)
    (elif (== OtherActor (Variables|Default|GetHomingTarget))
      (goto _label))))

(event EventBeginPlay
  (bind _projectilemovement (Variables|Default|GetProjectileMovement))
  (bind _homingtarget (Variables|Default|GetHomingTarget))
  (Utilities|IsValid _homingtarget
    (:Is%20Valid
      (Variables|/Script/Engine.ProjectileMovementComponent|SetHomingTargetComponent _projectilemovement (Variables|/Script/Engine.Actor|GetRootComponent _homingtarget)))
    (:Is%20Not%20Valid
      (Variables|/Script/Engine.ProjectileMovementComponent|SetbIsHomingProjectile _projectilemovement false)
      (Actor|SetLifeSpan 3.0))))

(fn ConstructionScript)