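; Music controller that plays an FMOD music event in 2D on BeginPlay and stops and releases it on EndPlay.
; ChangeMusic drives the event's "Level Section" parameter and, when asked to persist, saves the value in BP_GameInstance.
; The initial section comes from either that saved value or its own StartLevelSection, chosen by a flag.
; StopMusic also stops and releases the instance on demand.
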(event EventBeginPlay
  (bind _returnvalue (Class|FMODBlueprintStatics|PlayEvent2D (Variables|Default|GetMusicEvent)))
  (Variables|Default|SetMusicEventInstance _returnvalue)
  (bind _asbp_game_instance (Utilities|Casting|CastToBP_GameInstance (Game|GetGameInstance)))
  (Variables|Default|SetAs%20BP%20Game%20Instance _asbp_game_instance)
  (if (Variables|Default|GetStartFromGILevelSection)
    (CallFunction|ChangeMusic (Variables|/Game/Blueprints/Game/BP_GameInstance.BP_GameInstance_C|GetAudioLevelSection (Variables|Default|GetAs%20BP%20Game%20Instance)) true)
    (else
      (CallFunction|ChangeMusic (Variables|Default|GetStartLevelSection) false))))

(event EventEndPlay
  (params (EndPlayReason :type EEndPlayReason%20Enum :default "Destroyed"))
  (Class|FMODBlueprintStatics|EventInstanceStop (Variables|Default|GetMusicEventInstance) true))

(fn ConstructionScript)

(fn ChangeMusic
  (params (LevelSection :type Float%20%28double-precision%29) (Persist :type Boolean))
  (Class|FMODBlueprintStatics|EventInstanceSetParameter (Variables|Default|GetMusicEventInstance) "Level Section" LevelSection)
  (if Persist
    (Variables|/Game/Blueprints/Game/BP_GameInstance.BP_GameInstance_C|SetAudioLevelSection (Variables|Default|GetAs%20BP%20Game%20Instance) LevelSection)))

(fn StopMusic
  (Class|FMODBlueprintStatics|EventInstanceStop (Variables|Default|GetMusicEventInstance) true))