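; BP_MusicTrigger is a trigger volume that switches the music to its LevelSection when the hero enters it.
; On BeginPlay it looks up the BP_MusicController actor and caches it, re-calling the lookup immediately, with no delay, until one is valid.
; A Box overlap by BP_Hero calls ChangeMusic on that controller with Persist enabled.
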(event OnComponentBeginOverlap(Box)
  (params (OverlappedComponent :type Primitive%20Component%20Object%20Reference) (OtherActor :type Actor%20Object%20Reference) (OtherComp :type Primitive%20Component%20Object%20Reference) (OtherBodyIndex :type Integer) (bFromSweep :type Boolean) (SweepResult :type Hit%20Result%20Structure%20%28by%20ref%29))
  (bind _musiccontroller (Variables|Default|GetMusicController))
  (Utilities|Casting|CastToBP_Hero OtherActor)
  (Utilities|IsValid _musiccontroller
    (:Is%20Valid
      (Default|ChangeMusic _musiccontroller (Variables|Default|GetLevelSection) true))))

(event Custom|GetMusicController
  (bind _returnvalue (Actor|GetActorOfClass "/Game/Blueprints/Audio/BP_MusicController.BP_MusicController_C"))
  (Utilities|IsValid _returnvalue
    (:Is%20Valid
      (Variables|Default|SetMusicController _returnvalue))
    (:Is%20Not%20Valid
      (CallFunction|GetMusicController))))

(event EventBeginPlay
  (CallFunction|GetMusicController))

(fn ConstructionScript)