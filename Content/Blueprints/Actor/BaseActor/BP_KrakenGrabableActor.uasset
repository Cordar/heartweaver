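; BP_KrakenGrabableActor is an actor that can be targeted by the hero, by its name as something for the Kraken to grab.
; SetAsTargetIfHero and UnsetAsTargetIfHero forward to SetAsTarget and UnsetAsTarget only when the character's class is exactly BP_Hero, so subclasses do not pass.
; The WasSetasTarget and WasUnsetasTarget events show and hide its Widget component without propagating to children.
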(event EventBeginPlay)

(event Collision|EventActorBeginOverlap
  (params (OtherActor :type Actor%20Object%20Reference)))

(event EventTick
  (params (DeltaSeconds :type Float%20%28single-precision%29)))

(event EventWasSetasTarget
  (Rendering|SetVisibility (Variables|Default|GetWidget) true false))

(event EventWasUnsetasTarget
  (Rendering|SetVisibility (Variables|Default|GetWidget) false false))

(fn ConstructionScript)

(fn SetasTargetifHero
  (params (TargetCharacter :type Actor%20Object%20Reference))
  (if (== (Utilities|GetClass TargetCharacter) "/Game/Blueprints/Character/Hero/BP_Hero.BP_Hero_C")
    (Class|KrakenInteractableActor|SetasTarget TargetCharacter)))

(fn UnsetasTargetifHero
  (params (TargetCharacter :type Actor%20Object%20Reference))
  (if (== (Utilities|GetClass TargetCharacter) "/Game/Blueprints/Character/Hero/BP_Hero.BP_Hero_C")
    (Class|KrakenInteractableActor|UnsetasTarget TargetCharacter)))