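; BP_KrakenInteractableActor is a base interactable actor that shows an on-screen widget while it is targeted.
; Being set as target or deactivated creates the WidgetClass widget for player 0 and adds it to the viewport.
; Being untargeted or activated removes that widget.
; Helper functions set or unset the actor as target only when the supplied character casts to KrakenCharacter.
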(event EventWasSetasTarget
  (CallFunction|CreateWidget))

(event EventWasUnsetasTarget
  (CallFunction|RemoveWidget))

(event EventActivate
  (params (Instigator :type Actor%20Object%20Reference))
  (CallFunction|RemoveWidget))

(event EventDeactivate
  (CallFunction|CreateWidget))

(fn ConstructionScript)

(fn SetasTargetifHero
  (params (TargetCharacter :type Actor%20Object%20Reference))
  (bind _askraken_character (Utilities|Casting|CastToKrakenCharacter TargetCharacter))
  (Class|KrakenInteractableActor|SetasTarget _askraken_character))

(fn UnsetasTargetifHero
  (params (TargetCharacter :type Actor%20Object%20Reference))
  (bind _askraken_character (Utilities|Casting|CastToKrakenCharacter TargetCharacter))
  (Class|KrakenInteractableActor|UnsetasTarget _askraken_character))

(fn RemoveWidget
  (bind _widget (Variables|Default|GetWidget))
  (Utilities|IsValid _widget
    (:Is%20Valid
      (Widget|RemovefromParent _widget))))

(fn CreateWidget
  (bind _returnvalue (UserInterface|CreateWidget (Variables|Default|GetWidgetClass) (Game|GetPlayerController 0)))
  (bind _output_get (Variables|Default|SetWidget _returnvalue))
  (UserInterface|Viewport|AddtoViewport _output_get 0))