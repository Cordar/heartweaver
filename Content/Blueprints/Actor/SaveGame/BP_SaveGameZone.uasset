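; BP_SaveGameZone is a trigger actor that acts as a save point when the hero enters it.
; On Box overlap by a BP_Hero, it sets the game instance's PlayerLocation to the Arrow's world location, raised by the player capsule's half height.
; It then calls SaveGame on BP_GameInstance, so the saved position is the Arrow marker rather than where the player touched the box.
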(event OnComponentBeginOverlap(Box)
  (params (OverlappedComponent :type Primitive%20Component%20Object%20Reference) (OtherActor :type Actor%20Object%20Reference) (OtherComp :type Primitive%20Component%20Object%20Reference) (OtherBodyIndex :type Integer) (bFromSweep :type Boolean) (SweepResult :type Hit%20Result%20Structure%20%28by%20ref%29))
  (Utilities|Casting|CastToBP_Hero OtherActor)
  (bind _asbp_game_instance (Utilities|Casting|CastToBP_GameInstance (Game|GetGameInstance)))
  (Variables|/Game/Blueprints/Game/BP_GameInstance.BP_GameInstance_C|SetPlayerLocation _asbp_game_instance (+ (Transformation|GetWorldLocation (Variables|Default|GetArrow)) (Math|Vector|MakeVector 0.0 0.0 (Components|Capsule|GetScaledCapsuleHalfHeight (Variables|/Script/Engine.Character|GetCapsuleComponent (Game|GetPlayerCharacter 0))))))
  (Default|SaveGame _asbp_game_instance))

(fn ConstructionScript)