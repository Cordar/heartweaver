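; Sadness cloud actor that grows on spawn and hovers above a followed actor, turning toward that actor's follow camera.
; Tick lerps location and rotation in the target's local frame and fast-forwards the active Niagara rain simulation.
; SadnessActivated sets follow strengths, starts the rain and plays the Sadness audio event.
; EndCloudLife stops rain and audio, then shrinks and raises the cloud via timeline before destroying it.
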(event Custom|SadnessActivated
  ;[0.01096 0.01161 0.0137] On sadness activate
  (Variables|Default|SetFollowStrength 5.0)
  (Variables|Default|SetRotationStrength 5.0)
  (Components|Activation|Activate (Variables|Default|GetNS_SadnessCloudRain) true)
  (bind _returnvalue (Class|FMODBlueprintStatics|PlayEventatLocation "/Game/FMOD/Events/SFX/Player/Ability/Ability/Sadness.Sadness" (Transformation|GetActorTransform)))
  (Class|FMODBlueprintStatics|EventInstancePlay _returnvalue))

(event Custom|EndCloudLife
  (bind _returnvalue (Transformation|GetActorLocation))
  (Components|Activation|Deactivate (Variables|Default|GetNS_SadnessCloudRain))
  (Variables|Default|SetInitialScale (Variables|Default|GetFinalScale))
  (Variables|Default|SetInitialZLocation (.z (Transformation|GetActorLocation)))
  (bind _shrink (Timeline|ShrinkTimeline PlayFromStart)
    (:Update
      (Transformation|SetRelativeScale3D (Variables|Default|GetStaticMesh) (Math|Vector|Lerp(Vector) (Variables|Default|GetInitialScale) "0, 0, 0" _shrink))
      (Transformation|SetActorLocation (Math|Vector|MakeVector (.x _returnvalue) (.y _returnvalue) (Math|Float|Lerp (Variables|Default|GetInitialZLocation) (+ (Variables|Default|GetInitialZLocation) 3e+02) _shrink)) false true)
      (Class|FMODBlueprintStatics|EventInstanceStop (stale Custom|SadnessActivated _returnvalue) true))
    (:Finished
      (Actor|DestroyActor))))

(event EventBeginPlay
  ;[0.01096 0.01161 0.0137] Begin play
  (Variables|Default|SetInitialScale (Variables|/Script/Engine.SceneComponent|GetRelativeScale3D (Variables|Default|GetStaticMesh)))
  (bind _grow (Timeline|Timeline PlayFromStart)
    (:Update
      (Transformation|SetRelativeScale3D (Variables|Default|GetStaticMesh) (Math|Vector|Lerp(Vector) (Variables|Default|GetInitialScale) (Variables|Default|GetFinalScale) _grow)))))

(event EventTick
  (params (DeltaSeconds :type Float%20%28single-precision%29))
  (bind _actortofollow (Variables|Default|GetActorToFollow))
  (bind _ns_sadnesscloudrain (Variables|Default|GetNS_SadnessCloudRain))
  (bind _returnvalue (Transformation|GetActorTransform _actortofollow))
  (Utilities|IsValid _actortofollow
    (:Is%20Valid
      (Transformation|SetActorLocation (Math|Vector|Lerp(Vector) (Transformation|GetActorLocation) (Math|Transform|TransformLocation (Transformation|GetActorTransform _actortofollow) "0.000000,0.000000,300.000000") (* DeltaSeconds (Variables|Default|GetFollowStrength))) false true)
      (Transformation|SetActorRotation (Math|Rotator|Lerp(Rotator) (Transformation|GetActorRotation) (Math|Transform|TransformRotation _returnvalue (Math|Rotator|FindLookatRotation (Math|Transform|InverseTransformLocation _returnvalue (Transformation|GetActorLocation)) (Math|Transform|InverseTransformLocation _returnvalue (Transformation|GetActorLocation (Variables|/Script/HeartWeaver.KrakenCharacter|GetFollowCamera _actortofollow))))) (* DeltaSeconds (Variables|Default|GetRotationStrength)) true) true)
      (if (and (Utilities|IsValid _ns_sadnesscloudrain) (Components|Activation|IsActive _ns_sadnesscloudrain))
        (Class|NiagaraComponent|AdvanceSimulationbyTime _ns_sadnesscloudrain (* DeltaSeconds 1e+01) DeltaSeconds)))))

(fn ConstructionScript)