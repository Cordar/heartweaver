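; BP_FeelConnector_Sadness is a connectable actor for the Sadness feeling that also responds to gravity flips.
; On activation it plays a 2D Sadness event and tries to activate the player KrakenCharacter's abilities matching its gameplay tags.
; It binds to the GES gravity-switch tag event between BeginPlay and EndPlay, with a handler that toggles its flipped state.
; When gravity affects it, Tick moves it up or down by a fixed swept offset, independent of delta time.
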(event Custom|SwitchGravity
  (params (WildcardProperty :type GES%20Wildcard%20Property%20Structure%20%28by%20ref%29))
  (Variables|Default|SetIsGravityFlipped (not (Variables|Default|GetIsGravityFlipped))))

(event EventBeginPlay
  (Class|GlobalEventSystemBPLibrary|GESBindTagEventtoDelegate "(TagName=\"Event.Gravity.Switch\")" (EventDispatchers|CreateEvent :!event Custom|SwitchGravity)))

(event EventEndPlay
  (params (EndPlayReason :type EEndPlayReason%20Enum :default "Destroyed"))
  (Class|GlobalEventSystemBPLibrary|GESUnbindTagDelegate "(TagName=\"Event.Gravity.Switch\")" (EventDispatchers|CreateEvent :!event Custom|SwitchGravity)))

(event EventTick
  (params (DeltaSeconds :type Float%20%28single-precision%29))
  (if (Variables|Default|GetShouldGravityAffect)
    (if (Variables|Default|GetIsGravityFlipped)
      (Transformation|AddActorWorldOffset "0.000000,0.000000,10.000000" true)
      (else
        (Transformation|AddActorWorldOffset "0.000000,0.000000,-10.000000" true)))))

(event EventActivate
  (params (Instigator :type Actor%20Object%20Reference))
  (Class|FMODBlueprintStatics|PlayEvent2D "/Game/FMOD/Events/SFX/Player/Ability/Ability/Sadness.Sadness")
  (bind _askraken_character (Utilities|Casting|CastToKrakenCharacter (Game|GetPlayerCharacter 0)))
  (Abilities|TryActivateAbilitiesbyTag (Ability|GetAbilitySystemComponent _askraken_character) (GameplayTags|MakeGameplayTagContainerfromArray (Variables|Default|GetGameplay%20Tags)) true))

(fn ConstructionScript)