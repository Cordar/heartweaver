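; BP_CorruptedMesh is a connectable actor showing a corrupted mesh that dissolves away when activated.
; Construction adds a slightly enlarged copy of the assigned mesh with the corruption material and custom depth stencil.
; One-shot Activate waits briefly, puts a dynamic dissolve material on the root's first child mesh and animates DissolveAmount by timeline.
; On finish it destroys that component, calls CallFinishedActivation and expires; a Cover timeline is unused.
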(event Custom|UpdateMesh
  (Components|StaticMesh|SetStaticMesh (Variables|Default|GetStaticMeshComponent) (Variables|Default|GetStaticMesh)))

(event EventBeginPlay
  (bind _asstatic_mesh_component (Utilities|Casting|CastToStaticMeshComponent (Components|GetChildComponent (Variables|Transformation|GetRootComponent) 0)))
  (Variables|Default|SetDissolveMesh _asstatic_mesh_component)
  (Class|NiagaraFunctionLibrary|OverrideSystemUserVariableStaticMeshComponent)
  (Variables|Default|SetOriginalMaterial (Rendering|Material|GetMaterial (Variables|Default|GetStaticMesh) 0)))

(event EventActivate
  (params (Instigator :type Actor%20Object%20Reference))
  (if (not (Variables|Default|GetActivated))
    (Variables|Default|SetActivated true)
    (Utilities|FlowControl|Delay 0.25)
    (bind _returnvalue (Rendering|Material|CreateDynamicMaterialInstance (Variables|Default|GetDissolveMesh) 0 (Variables|Default|GetDissolveCorruptionMaterial) "None" :!class /Script/Engine.PrimitiveComponent))
    (Variables|Default|SetDynMaterial _returnvalue)
    (bind _dissolve (Timeline|Dissolve Play)
      (:Update
        (Rendering|Material|SetScalarParameterValue (Variables|Default|GetDynMaterial) "DissolveAmount" _dissolve :!class /Script/Engine.MaterialInstanceDynamic))
      (:Finished
        (Components|DestroyComponent (Variables|Default|GetDissolveMesh))
        (Default|CallFinishedActivation)
        (Actor|SetLifeSpan 1.0)))))

(fn ConstructionScript
  (bind _returnvalue (AddComponent|AddStaticMeshComponent false))
  (Utilities|IsValid _returnvalue
    (:Is%20Valid
      (Variables|Default|SetStaticMeshComponent _returnvalue)
      (Components|StaticMesh|SetStaticMesh _returnvalue (Variables|Default|GetStaticMesh))
      (Transformation|SetRelativeScale3D _returnvalue "1.010000,1.010000,1.010000")
      (Rendering|Material|SetMaterial _returnvalue 0 (Variables|Default|GetCorruptionMaterial))
      (Rendering|SetRenderCustomDepth _returnvalue true)
      (Rendering|SetCustomDepthStencilValue _returnvalue 1))))