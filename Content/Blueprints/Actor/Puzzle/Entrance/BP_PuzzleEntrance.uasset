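; Puzzle entrance actor that moves the player into a streamed puzzle level when activated.
; On BeginPlay it asks BP_GameInstance whether its puzzle is solved, and if so fires OnPuzzleSolved and destroys itself.
; Activate shows a loading widget, streams in the puzzle level, moves the player to its capsule and switches music.
; It then unloads the surrounding sublevels, removing the widget just before unloading Gameplay last.
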(event EventBeginPlay
  (CallFunction|GetGameInstance)
  (CallFunction|CheckifPuzzleIsSolved))

(event EventActivate
  (params (Instigator :type Actor%20Object%20Reference))
  (bind _musiccontroller (Variables|Default|GetMusicController))
  (bind _returnvalue (UserInterface|CreateWidget "/Game/Blueprints/UI/Widget/LoadingScreen/BPW_Loading.BPW_Loading_C" (Game|GetPlayerController 0)))
  (bind _output_get (Variables|Default|SetLoadingWidget _returnvalue))
  (UserInterface|Viewport|AddtoViewport _output_get 0)
  (Class|GameplayStatics|LoadStreamLevelbySoftObjectPtr (Variables|Default|GetPuzzleLevel) true false)
  (Transformation|SetActorLocation (Game|GetPlayerCharacter 0) (Transformation|GetWorldLocation (Variables|Default|GetCapsule)) false false)
  (if (Utilities|IsValidSoftObjectReference _musiccontroller)
    (Default|ChangeMusic (Utilities|ResolveSoftReference _musiccontroller) (Variables|Default|GetMusicLevelSection) true))
  (Class|GameplayStatics|UnloadStreamLevelbySoftObjectPtr "/Game/Maps/Numbness/Sublevels/Environment.Environment" false)
  (Class|GameplayStatics|UnloadStreamLevelbySoftObjectPtr "/Game/Maps/Numbness/Sublevels/Camera.Camera" false)
  (Class|GameplayStatics|UnloadStreamLevelbySoftObjectPtr "/Game/Maps/Numbness/Sublevels/Lighting.Lighting" false)
  (Class|GameplayStatics|UnloadStreamLevelbySoftObjectPtr "/Game/Maps/Numbness/Sublevels/UI.UI" false)
  (Class|GameplayStatics|UnloadStreamLevelbySoftObjectPtr "/Game/Maps/Numbness/Sublevels/Music.Music" false)
  (Widget|RemovefromParent (Variables|Default|GetLoadingWidget))
  (Class|GameplayStatics|UnloadStreamLevelbySoftObjectPtr "/Game/Maps/Numbness/Sublevels/Gameplay.Gameplay" false))

(fn ConstructionScript)

(fn CheckifPuzzleIsSolved
  (bind _issolved (Default|IsPuzzleSolved (Variables|Default|GetAs%20BP%20Game%20Instance) (Variables|Default|GetPuzzle)))
  (if _issolved
    (Default|CallOnPuzzleSolved)
    (Actor|DestroyActor)))

(fn GetGameInstance
  (bind _asbp_game_instance (Utilities|Casting|CastToBP_GameInstance (Game|GetGameInstance)))
  (Variables|Default|SetAs%20BP%20Game%20Instance _asbp_game_instance))