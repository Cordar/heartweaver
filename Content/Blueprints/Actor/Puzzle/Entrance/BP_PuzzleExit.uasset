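; BP_PuzzleExit is a puzzle exit actor that returns the player to the main world and records the puzzle as solved.
; On Activate it shows a loading widget and streams in the world's sublevels, from environment to gameplay.
; It then restores the player's location from the game instance and saves.
; If the soft-referenced entrance resolves, it notifies it, removes the widget and unloads the puzzle level.
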(event EventActivate
  (params (Instigator :type Actor%20Object%20Reference))
  (bind _puzzleentrance (Variables|Default|GetPuzzleEntrance))
  (bind _returnvalue (UserInterface|CreateWidget "/Game/Blueprints/UI/Widget/LoadingScreen/BPW_Loading.BPW_Loading_C" (Game|GetPlayerController 0)))
  (bind _output_get (Variables|Default|SetLoadingWidget _returnvalue))
  (UserInterface|Viewport|AddtoViewport _output_get 0)
  (Class|GameplayStatics|LoadStreamLevelbySoftObjectPtr "/Game/Maps/Numbness/Sublevels/Environment.Environment" true false)
  (Class|GameplayStatics|LoadStreamLevelbySoftObjectPtr "/Game/Maps/Numbness/Sublevels/Camera.Camera" true false)
  (Class|GameplayStatics|LoadStreamLevelbySoftObjectPtr "/Game/Maps/Numbness/Sublevels/ExpensiveStuff.ExpensiveStuff" true false)
  (Class|GameplayStatics|LoadStreamLevelbySoftObjectPtr "/Game/Maps/Numbness/Sublevels/Lighting.Lighting" true false)
  (Class|GameplayStatics|LoadStreamLevelbySoftObjectPtr "/Game/Maps/Numbness/Sublevels/UI.UI" true false)
  (Class|GameplayStatics|LoadStreamLevelbySoftObjectPtr "/Game/Maps/Numbness/Sublevels/Music.Music" true false)
  (Class|GameplayStatics|LoadStreamLevelbySoftObjectPtr "/Game/Maps/Numbness/Sublevels/Gameplay.Gameplay" true false)
  (bind _asbp_game_instance (Utilities|Casting|CastToBP_GameInstance (Game|GetGameInstance)))
  (Transformation|SetActorLocation (Game|GetPlayerCharacter 0) (Variables|/Game/Blueprints/Game/BP_GameInstance.BP_GameInstance_C|GetPlayerLocation _asbp_game_instance) false false)
  (Default|MarkPuzzleasSolved _asbp_game_instance (Variables|Default|GetPuzzleSolved))
  (Default|SaveGame _asbp_game_instance)
  (Utilities|IsValid (Utilities|ResolveSoftReference _puzzleentrance)
    (:Is%20Valid
      (Default|CallOnPuzzleSolved (Utilities|ResolveSoftReference _puzzleentrance))
      (Widget|RemovefromParent (Variables|Default|GetLoadingWidget))
      (Class|GameplayStatics|UnloadStreamLevelbySoftObjectPtr (Variables|Default|GetCurrentPuzzle) false))))

(fn ConstructionScript)