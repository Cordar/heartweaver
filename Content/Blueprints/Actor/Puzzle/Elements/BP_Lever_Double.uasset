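; Two-way puzzle lever that the player, the companion or another instigator toggles between active and inactive.
; Activation snaps the player to the arrow for the current state, disables movement and plays the matching pull montage, while the companion plays a lash montage.
; Montage notifies, companion interruption or other instigators drive a rotation timeline that flips the state and fires activated or deactivated calls when finished.
; A box overlap sets or unsets it as the hero's target.
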(event OnComponentBeginOverlap(Box)
  (params (OverlappedComponent :type Primitive%20Component%20Object%20Reference) (OtherActor :type Actor%20Object%20Reference) (OtherComp :type Primitive%20Component%20Object%20Reference) (OtherBodyIndex :type Integer) (bFromSweep :type Boolean) (SweepResult :type Hit%20Result%20Structure%20%28by%20ref%29))
  (CallFunction|SetasTargetifHero OtherActor))

(event OnComponentEndOverlap(Box)
  (params (OverlappedComponent :type Primitive%20Component%20Object%20Reference) (OtherActor :type Actor%20Object%20Reference) (OtherComp :type Primitive%20Component%20Object%20Reference) (OtherBodyIndex :type Integer))
  (CallFunction|UnsetasTargetifHero OtherActor))

(event EventActivate
  (params (Instigator :type Actor%20Object%20Reference))
  (bind _returnvalue (Game|GetPlayerCharacter 0))
  (if (Variables|Default|GetIsActive)
    (Variables|Default|SetMontage%20to%20Play "/Game/Assets/Character/Ace/Animation/Montage/AM_Ace_Lever_Reverse.AM_Ace_Lever_Reverse")
    (Variables|Default|SetArrowForPosition (Variables|Default|GetArrow_Reverse))
    (else
      (Variables|Default|SetMontage%20to%20Play "/Game/Assets/Character/Ace/Animation/Montage/AM_Ace_Lever.AM_Ace_Lever")
      (Variables|Default|SetArrowForPosition (Variables|Default|GetArrow))))
  (if (== Instigator _returnvalue)
    (Class|BPIHero|DisableMovement(Message) _returnvalue)
    (Transformation|SetActorLocationAndRotation _returnvalue (Math|Vector|MakeVector (.x (Transformation|GetWorldLocation (Variables|Default|GetArrowForPosition))) (.y (Transformation|GetWorldLocation (Variables|Default|GetArrowForPosition))) (.z (Transformation|GetActorLocation _returnvalue))) (Transformation|GetWorldRotation (Variables|Default|GetArrowForPosition)) false true)
    (Animation|Montage|PlayMontage (Variables|/Script/Engine.Character|GetMesh _returnvalue) (Variables|Default|GetMontage%20to%20Play)
      (:OnCompleted
        (Class|BPIHero|EnableMovement(Message) _returnvalue))
      (:OnNotifyBegin
        (if (Variables|Default|GetIsActive) :!label _label
          (bind _rotation (Timeline|Rotation Reverse)
            (:Update
              (Transformation|SetRelativeRotation (Variables|Default|GetLever) (Math|Rotator|Lerp(Rotator) "0.000000,0.000000,10.000000" "0.000000,0.000000,35.000000" _rotation) false false))
            (:Finished
              (if (Variables|Default|GetIsActive)
                (Variables|Default|SetIsActive false)
                (Default|CallDeactivated)
                (else
                  (Variables|Default|SetIsActive true)
                  (Default|CallActivated)))))
          (else
            (Timeline|Rotation Play)))))
    (else
      (bind _asbp_companion (Utilities|Casting|CastToBP_Companion Instigator)
        (:then
          (Animation|Montage|PlayMontage (Variables|/Script/Engine.Character|GetMesh _asbp_companion) "/Game/Assets/Character/Mark/Animations/AM_Mark_Lash.AM_Mark_Lash"
            (:OnInterrupted
              (goto _label))
            (:OnNotifyBegin
              (goto _label))))
        (:CastFailed
          (goto _label))))))

(fn ConstructionScript
  (|CallParentFunction))