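; Pushable puzzle object that follows global gravity switches, flipping over and moving up or down each tick with sweeps.
; Construction sets the mesh and adds an arrow for each designer-defined push transform.
; Hold finds the nearest in-range transform, validates floor and line of sight for either gravity direction, then snaps the character there and starts KrakenPushComponent's push.
; AddForce slides the object by an offset on a timeline, suspending gravity until finished.
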(event Custom|SwitchGravity
  (params (WildcardProperty :type GES%20Wildcard%20Property%20Structure%20%28by%20ref%29))
  (Variables|Default|SetIsGravityFlipped (not (Variables|Default|GetIsGravityFlipped)))
  (Transformation|AddActorLocalRotation "0.000000,0.000000,180.000000" true false))

(event Custom|AddForce
  (params (DeltaLocation :type Vector))
  (Variables|Default|SetIsGravityActive false)
  (Variables|Default|SetFinalLocation (+ DeltaLocation (Transformation|GetActorLocation)))
  (Variables|Default|SetInitialLocation (Transformation|GetActorLocation))
  (bind _distance (Timeline|Move PlayFromStart)
    (:Update
      (Transformation|SetActorLocation (Math|Vector|Lerp(Vector) (Variables|Default|GetInitialLocation) (Variables|Default|GetFinalLocation) _distance) true false))
    (:Finished
      (Variables|Default|SetIsGravityActive true))))

(event EventBeginPlay
  (Class|GlobalEventSystemBPLibrary|GESBindTagEventtoDelegate "(TagName=\"Event.Gravity.Switch\")" (EventDispatchers|CreateEvent :!event Custom|SwitchGravity)))

(event Collision|EventActorBeginOverlap
  (params (OtherActor :type Actor%20Object%20Reference)))

(event EventTick
  (params (DeltaSeconds :type Float%20%28single-precision%29))
  (if (Variables|Default|GetIsGravityActive)
    (if (Variables|Default|GetIsGravityFlipped)
      (Transformation|AddActorWorldOffset "0.000000,0.000000,10.000000" true)
      (else
        (Transformation|AddActorWorldOffset "0.000000,0.000000,-10.000000" true)))))

(event EventHold
  (params (Character :type Kraken%20Character%20Object%20Reference))
  (CallFunction|HandleInteraction Character))

(event EventEndPlay
  (params (EndPlayReason :type EEndPlayReason%20Enum :default "Destroyed"))
  (Class|GlobalEventSystemBPLibrary|GESUnbindTagDelegate "(TagName=\"Event.Gravity.Switch\")" (EventDispatchers|CreateEvent :!event Custom|SwitchGravity)))

(fn ConstructionScript
  (bind _newmesh (Variables|Default|GetNewMesh))
  (bind _staticmesh (Variables|Default|GetStaticMesh))
  (Components|StaticMesh|SetStaticMesh _staticmesh _newmesh)
  (Rendering|Material|SetMaterial _staticmesh 0 (Rendering|Material|GetMaterial _newmesh 0))
  (for _array_element (Variables|Default|GetPushTransform)
    (AddComponent|AddArrowComponent false _array_element)))

(fn HandleInteraction
  (params (Character :type Kraken%20Character%20Object%20Reference))
  (bind _returnvalue (Actor|GetComponentbyClass Character "/Script/HeartWeaver.KrakenPushComponent"))
  (bind _returnvalue_2 (Transformation|GetActorTransform Character))
  (bind _capsulecomponent (Variables|/Script/Engine.Character|GetCapsuleComponent Character))
  (bind _capsulecomponent_2 (Variables|/Script/Engine.Character|GetCapsuleComponent Character))
  (bind _capsulecomponent_3 (Variables|/Script/Engine.Character|GetCapsuleComponent Character))
  (bind _returnvalue_3 (Components|Capsule|GetScaledCapsuleHalfHeight _capsulecomponent_2))
  (Utilities|IsValid Character
    (:Is%20Valid
      (Utilities|IsValid _returnvalue
        (:Is%20Valid
          (LocalVariables|SetPushComponent _returnvalue)
          (bind _bestindex (CallFunction|FindClosestPushTransformIndex (Math|Conversions|ToVector2D(Vector) (Transformation|GetActorLocation Character)) (Variables|/Script/HeartWeaver.KrakenPushComponent|GetPushRange (LocalVariables|GetPushComponent))))
          (if (!= _bestindex -1)
            (if (<= (.z (Variables|/Script/Engine.CharacterMovementComponent|GetGravityDirection (Variables|/Script/HeartWeaver.KrakenCharacter|GetKrakenCharacterMovementComponent Character))) 0.0)
              (LocalVariables|SetCharacterNewTransform (Math|Transform|MakeTransform (+ (.location (Math|Transform|ComposeTransforms (Utilities|Array|Get(acopy) (Variables|Default|GetPushTransform) _bestindex) (Transformation|GetActorTransform))) (Math|Vector|MakeVector 0.0 0.0 _returnvalue_3)) (.rotation (Math|Transform|ComposeTransforms (Utilities|Array|Get(acopy) (Variables|Default|GetPushTransform) _bestindex) (Transformation|GetActorTransform))) (.scale _returnvalue_2)))
              (bind (_outhit _returnvalue_4) (Collision|CapsuleTraceByChannel (+ (.location (LocalVariables|GetCharacterNewTransform)) "0.000000,0.000000,100.000000") (- (.location (LocalVariables|GetCharacterNewTransform)) "0.000000,0.000000,100.000000") (Components|Capsule|GetScaledCapsuleRadius _capsulecomponent) (Components|Capsule|GetScaledCapsuleHalfHeight _capsulecomponent) "TraceTypeQuery1" false 0 "None"))
              (if _returnvalue_4
                (if (<= (Class|CharacterMovementComponent|GetWalkableFloorZ (Variables|/Script/Engine.Character|GetCharacterMovement Character)) (.Z (Math|Vector|BreakVector (.impactnormal _outhit))))
                  (bind (_outhit_2 _returnvalue_5) (Collision|LineTraceByChannel (Transformation|GetActorLocation) (.location (LocalVariables|GetCharacterNewTransform)) "TraceTypeQuery1" false (Utilities|Array|MakeArray Character) "None" :!label _label))
                  (LocalVariables|SetNewLocalVar _outhit_2)
                  (if (not _returnvalue_5)
                    (Transformation|SetActorTransform Character (LocalVariables|GetCharacterNewTransform))
                    (Class|KrakenPushComponent|BeginPush (LocalVariables|GetPushComponent) self)
                    (else
                      (Development|PrintString "WallsBetweenCharacter  And Object")))
                  (else
                    (Development|PrintString "Floor Is Not Walkable")))
                (else
                  (Development|PrintString "No Room To Stand")))
              (else
                (LocalVariables|SetCharacterNewTransform (Math|Transform|MakeTransform (- (.location (Math|Transform|ComposeTransforms (Utilities|Array|Get(acopy) (Variables|Default|GetPushTransform) _bestindex) (Transformation|GetActorTransform))) (Math|Vector|MakeVector 0.0 0.0 _returnvalue_3)) (.rotation (Math|Transform|ComposeTransforms (Utilities|Array|Get(acopy) (Variables|Default|GetPushTransform) _bestindex) (Transformation|GetActorTransform))) (.scale _returnvalue_2)))
                (bind (_outhit_3 _returnvalue_6) (Collision|CapsuleTraceByChannel (- (.location (LocalVariables|GetCharacterNewTransform)) "0.000000,0.000000,100.000000") (+ (.location (LocalVariables|GetCharacterNewTransform)) "0.000000,0.000000,100.000000") (Components|Capsule|GetScaledCapsuleRadius _capsulecomponent_3) (Components|Capsule|GetScaledCapsuleHalfHeight _capsulecomponent_3) "TraceTypeQuery1" false 0 "None"))
                (if _returnvalue_6
                  (if (<= (.Z (Math|Vector|BreakVector (.impactnormal _outhit_3))) (Class|CharacterMovementComponent|GetWalkableFloorZ (Variables|/Script/Engine.Character|GetCharacterMovement Character)))
                    (goto _label)
                    (else
                      (Development|PrintString "Floor Is Not Walkable")))
                  (else
                    (Development|PrintString "No Room To Stand")))))
            (else
              (Development|PrintString "Push Transform Not Found"))))
        (:Is%20Not%20Valid
          (Development|PrintString "PushComponent not found in Character"))))
    (:Is%20Not%20Valid
      (Development|PrintString "Character Is Not Valid"))))

(fn FindClosestPushTransformIndex
  (params (CharacterLocation :type Vector%202D%20Structure) (PushRange :type Float%20%28double-precision%29))
  (for (_array_element _array_index) (Variables|Default|GetPushTransform)
    (LocalVariables|SetCurrentTransformIndex _array_index)
    (LocalVariables|SetCurrentDistanceSquared (Class|KismetMathLibrary|DistanceSquared2D (Math|Conversions|ToVector2D(Vector) (Math|Transform|TransformLocation (Transformation|GetActorTransform) (.location _array_element))) CharacterLocation))
    (if (<= (LocalVariables|GetCurrentDistanceSquared) (Math|Float|Square PushRange))
      (if (or (< (LocalVariables|GetCurrentDistanceSquared) (LocalVariables|GetClosestDistanceSquared)) (< (LocalVariables|GetClosestTransformIndex) 0))
        (LocalVariables|SetClosestTransformIndex (LocalVariables|GetCurrentTransformIndex))
        (LocalVariables|SetClosestDistanceSquared (LocalVariables|GetCurrentDistanceSquared)))))
  (return (LocalVariables|GetClosestTransformIndex)))