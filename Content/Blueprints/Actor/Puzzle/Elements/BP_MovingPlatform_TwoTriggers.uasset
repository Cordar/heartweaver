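; Moving platform puzzle element that needs several activations, judging by its name from two triggers, before it activates.
; Activate and Deactivate raise and lower a counter, calling the parent's Activate when it reaches NumberOfActivatesNeeded and the parent's Deactivate when it drops to one below.
; All other behavior is left to the parent class.
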(event EventBeginPlay
  (|CallParentFunction) ; This node is disabled and will not be called.\nDrag off pins to build functionality.
)

(event Collision|EventActorBeginOverlap
  (params (OtherActor :type Actor%20Object%20Reference)))

(event EventTick
  (params (DeltaSeconds :type Float%20%28single-precision%29)))

(event EventActivate
  (params (Instigator :type Actor%20Object%20Reference))
  (bind _result (Math|Integer|IncrementInt (Variables|Default|GetActivateCounter))
    (:%20%20
      (if (== _result (Variables|Default|GetNumberOfActivatesNeeded))
        (|CallParentFunction 0)))))

(event EventDeactivate
  (bind _result (Math|Integer|DecrementInt (Variables|Default|GetActivateCounter))
    (:%20%20
      (if (== _result (- (Variables|Default|GetNumberOfActivatesNeeded) 1))
        (|CallParentFunction)))))

(fn ConstructionScript
  (|CallParentFunction))