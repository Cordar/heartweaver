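; Double door puzzle element that swings open on Activate and closed on Deactivate.
; A timeline yaws the left and right pivots in opposite directions from rotations cached at BeginPlay, playing forward or in reverse.
; One 2D FMOD sound event is started on activation, paused when the timeline finishes and resumed on deactivation, with a DoorState parameter marking the direction.
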(event EventBeginPlay
  (|CallParentFunction)
  (Variables|Default|SetRotationDL (Variables|/Script/Engine.SceneComponent|GetRelativeRotation (Variables|Default|GetPivotL)))
  (Variables|Default|SetRotationDR (Variables|/Script/Engine.SceneComponent|GetRelativeRotation (Variables|Default|GetPivotR))))

(event EventDeactivate
  (Class|FMODBlueprintStatics|EventInstanceSetPaused (stale EventActivate _returnvalue) false)
  (Class|FMODBlueprintStatics|EventInstanceSetParameter (stale EventActivate _returnvalue) "DoorState" 1.0)
  (bind _newtrack_0 (Timeline|Door%20rotation Reverse)
    (:Update
      (Transformation|SetRelativeRotation (Variables|Default|GetPivotL) (Math|Rotator|CombineRotators (Variables|Default|GetRotationDL) (* (Math|Rotator|MakeRotator 0.0 0.0 _newtrack_0) -1.0)) false false)
      (Transformation|SetRelativeRotation (Variables|Default|GetPivotR) (Math|Rotator|CombineRotators (Math|Rotator|MakeRotator 0.0 0.0 _newtrack_0) (Variables|Default|GetRotationDR)) false false))
    (:Finished
      (Class|FMODBlueprintStatics|EventInstanceSetPaused (stale EventActivate _returnvalue) true))))

(event EventActivate
  (params (Instigator :type Actor%20Object%20Reference))
  (bind _returnvalue (Class|FMODBlueprintStatics|PlayEvent2D "/Game/FMOD/Events/SFX/Objects/Door/DoorOpenClose.DoorOpenClose"))
  (Class|FMODBlueprintStatics|EventInstanceSetParameter _returnvalue "DoorState" 0.0)
  (bind _newtrack_0 (Timeline|Door%20rotation Play)
    (:Update
      (Transformation|SetRelativeRotation (Variables|Default|GetPivotL) (Math|Rotator|CombineRotators (Variables|Default|GetRotationDL) (* (Math|Rotator|MakeRotator 0.0 0.0 _newtrack_0) -1.0)) false false)
      (Transformation|SetRelativeRotation (Variables|Default|GetPivotR) (Math|Rotator|CombineRotators (Math|Rotator|MakeRotator 0.0 0.0 _newtrack_0) (Variables|Default|GetRotationDR)) false false))
    (:Finished
      (Class|FMODBlueprintStatics|EventInstanceSetPaused _returnvalue true))))

(fn ConstructionScript)