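; BP_FeelingConnector is a puzzle element that temporarily switches on a linked Activable.
; Activate is guarded by IsActivated, sends the activate message to the Activable, calls the Activated event dispatcher and starts a one-shot timer.
; After SecondsToDeactivate, the timer fires Deactivate, which sends the deactivate message and clears the flag so the connector can be triggered again.
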(event EventDeactivate
  (Class|KrakenActivableObject|Deactivate(Message) (Variables|Default|GetActivable))
  (Variables|Default|SetIs%20Activated false))

(event EventActivate
  (params (Instigator :type Actor%20Object%20Reference))
  (if (not (Variables|Default|GetIs%20Activated))
    (Class|KrakenActivableObject|Activate(Message) (Variables|Default|GetActivable))
    (Variables|Default|SetIs%20Activated true)
    (Default|CallActivated)
    (Utilities|Time|SetTimerbyEvent (delegate EventDeactivate) (Variables|Default|GetSeconds%20To%20Deactivate))))

(fn ConstructionScript
  (|CallParentFunction))