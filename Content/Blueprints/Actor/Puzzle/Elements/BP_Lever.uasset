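; BP_Lever is a puzzle lever that the player, the companion Mark or other instigators can activate, with overlap-based hero targeting while inactive.
; The player snaps to an arrow with movement disabled for a montage, whose notify starts the rotation timeline.
; Mark switches AI state around a lash montage before triggering it.
; The timeline tilts the lever and toggles IsActive on finish, calling Activated or Deactivated; Deactivate plays it in reverse.
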(event OnComponentBeginOverlap(Box)
  (params (OverlappedComponent :type Primitive%20Component%20Object%20Reference) (OtherActor :type Actor%20Object%20Reference) (OtherComp :type Primitive%20Component%20Object%20Reference) (OtherBodyIndex :type Integer) (bFromSweep :type Boolean) (SweepResult :type Hit%20Result%20Structure%20%28by%20ref%29))
  (if (not (Variables|Default|GetIsActive))
    (CallFunction|SetasTargetifHero OtherActor)))

(event OnComponentEndOverlap(Box)
  (params (OverlappedComponent :type Primitive%20Component%20Object%20Reference) (OtherActor :type Actor%20Object%20Reference) (OtherComp :type Primitive%20Component%20Object%20Reference) (OtherBodyIndex :type Integer))
  (CallFunction|UnsetasTargetifHero OtherActor))

(event EventDeactivate
  (if (Variables|Default|GetIsActive)
    ;[0.6749 0.7151 0.8438] Acabamos la secuencia
    (bind _rotation (Timeline|Rotation Reverse)
      (:Update
        (Transformation|SetRelativeRotation (Variables|Default|GetLever) (Math|Rotator|Lerp(Rotator) "0.000000,0.000000,10.000000" "0.000000,0.000000,35.000000" _rotation) false false))
      (:Finished
        (if (Variables|Default|GetIsActive)
          (Variables|Default|SetIsActive false)
          (Default|CallDeactivated)
          (else
            (Variables|Default|SetIsActive true)
            (Default|CallActivated)))))))

(event EventActivate
  (params (Instigator :type Actor%20Object%20Reference))
  (bind _returnvalue (Game|GetPlayerCharacter 0))
  (bind _arrow (Variables|Default|GetArrow))
  (bind _returnvalue_2 (Transformation|GetWorldLocation _arrow))
  (if (not (Variables|Default|GetIsActive))
    (if (== Instigator _returnvalue)
      ;[0.6749 0.7151 0.8438] Evento de interacción del jugador
      (Class|BPIHero|DisableMovement(Message) _returnvalue)
      (Transformation|SetActorLocationAndRotation _returnvalue (Math|Vector|MakeVector (.x _returnvalue_2) (.y _returnvalue_2) (.z (Transformation|GetActorLocation _returnvalue))) (Transformation|GetWorldRotation _arrow) false true)
      (Animation|Montage|PlayMontage (Variables|/Script/Engine.Character|GetMesh _returnvalue) "/Game/Assets/Character/Ace/Animation/Montage/AM_Ace_Lever.AM_Ace_Lever"
        (:OnCompleted
          (Class|BPIHero|EnableMovement(Message) _returnvalue))
        (:OnNotifyBegin
          ;[0.6749 0.7151 0.8438] Acabamos la secuencia
          (bind _rotation (Timeline|Rotation Play)
            (:Update
              (Transformation|SetRelativeRotation (Variables|Default|GetLever) (Math|Rotator|Lerp(Rotator) "0.000000,0.000000,10.000000" "0.000000,0.000000,35.000000" _rotation) false false))
            (:Finished
              (if (Variables|Default|GetIsActive)
                (Variables|Default|SetIsActive false)
                (Default|CallDeactivated)
                (else
                  (Variables|Default|SetIsActive true)
                  (Default|CallActivated)))))))
      (else
        ;[0.6749 0.7151 0.8438] Evento de interacción de Mark
        (bind _asbp_companion (Utilities|Casting|CastToBP_Companion Instigator)
          (:then
            (Default|SetIAState (.AsBP%20Companion%20AIController (Utilities|Casting|CastToBP_CompanionAIController (AI|GetAIController _asbp_companion))) "NewEnumerator4")
            (Animation|Montage|PlayMontage (Variables|/Script/Engine.Character|GetMesh _asbp_companion) "/Game/Assets/Character/Mark/Animations/AM_Mark_Lash.AM_Mark_Lash"
              (:OnCompleted
                _)
              (:OnInterrupted
                _)
              (:OnNotifyBegin
                _))
            (Utilities|IsValid (.AsBP%20Companion%20AIController (Utilities|Casting|CastToBP_CompanionAIController (AI|GetAIController _asbp_companion)))
              (:Is%20Valid
                (Default|SetIAState (.AsBP%20Companion%20AIController (Utilities|Casting|CastToBP_CompanionAIController (AI|GetAIController _asbp_companion))) "NewEnumerator0")
                (Timeline|Rotation Play))))
          (:CastFailed
            (Timeline|Rotation Play)))))))

(fn ConstructionScript
  (|CallParentFunction))