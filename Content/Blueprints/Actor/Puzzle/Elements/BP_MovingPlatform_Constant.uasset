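; Puzzle platform that moves between its start and end transforms on a timeline whose play rate is set by Speed.
; Activate and Deactivate share one toggle that plays or stops the timeline, whose update interpolates location, rotation and scale.
; Each toggle triggers the FMOD "on" sound, and ActivatePlatformIfNeeded snaps an active platform to its end transform.
; Uncalled helpers can lock and restore hero movement; SPUD save overrides return defaults.
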(event Custom|ActivatePlatformIfNeeded
  (if (Variables|Default|GetIsActivated)
    (Transformation|SetActorTransform (Variables|Default|GetEndTransform))))

(event EventDeactivate
  (bind _starttransform (Variables|Default|GetStartTransform))
  (bind _endtransform (Variables|Default|GetEndTransform))
  (if (Variables|Default|GetIsActivated)
    (CallFunction|PlaySound true)
    (Variables|Default|SetIsActivated false)
    (bind (_direction _time _rotation) (Timeline|TimelineMove Stop)
      (:Update
        (Transformation|SetActorTransform (Math|Transform|MakeTransform (.location (Math|Transform|Lerp(Transform) (Math|Transform|MakeTransform (.location _starttransform) "0, 0, 0" (.scale _starttransform)) (Math|Transform|MakeTransform (.location _endtransform) "0, 0, 0" (.scale _endtransform)) _time)) (Math|Rotator|Lerp(Rotator) (.rotation _starttransform) (.rotation _endtransform) _rotation) (.scale (Math|Transform|Lerp(Transform) (Math|Transform|MakeTransform (.location _starttransform) "0, 0, 0" (.scale _starttransform)) (Math|Transform|MakeTransform (.location _endtransform) "0, 0, 0" (.scale _endtransform)) _time))))))
    (else
      (CallFunction|PlaySound true)
      (Variables|Default|SetIsActivated true)
      (Timeline|TimelineMove Play))))

(event EventBeginPlay
  (|CallParentFunction)
  (Variables|Default|SetStartTransform (Transformation|GetActorTransform))
  (Components|Timeline|SetPlayRate (Variables|Default|GetTimelineMove) (Variables|Default|GetSpeed)))

(event EventActivate
  (params (Instigator :type Actor%20Object%20Reference))
  (bind _starttransform (Variables|Default|GetStartTransform))
  (bind _endtransform (Variables|Default|GetEndTransform))
  (if (Variables|Default|GetIsActivated)
    (CallFunction|PlaySound true)
    (Variables|Default|SetIsActivated false)
    (bind (_direction _time _rotation) (Timeline|TimelineMove Stop)
      (:Update
        (Transformation|SetActorTransform (Math|Transform|MakeTransform (.location (Math|Transform|Lerp(Transform) (Math|Transform|MakeTransform (.location _starttransform) "0, 0, 0" (.scale _starttransform)) (Math|Transform|MakeTransform (.location _endtransform) "0, 0, 0" (.scale _endtransform)) _time)) (Math|Rotator|Lerp(Rotator) (.rotation _starttransform) (.rotation _endtransform) _rotation) (.scale (Math|Transform|Lerp(Transform) (Math|Transform|MakeTransform (.location _starttransform) "0, 0, 0" (.scale _starttransform)) (Math|Transform|MakeTransform (.location _endtransform) "0, 0, 0" (.scale _endtransform)) _time))))))
    (else
      (CallFunction|PlaySound true)
      (Variables|Default|SetIsActivated true)
      (Timeline|TimelineMove Play))))

(fn ConstructionScript)

(fn PlaySound
  (params (PlayActivateSound? :type Boolean))
  (if PlayActivateSound?
    (LocalVariables|SetFMODEvent "/Game/FMOD/Events/SFX/Objects/MovingPlattform/MovingPlattformOn.MovingPlattformOn")
    (LocalVariables|SetFMODEvent%20Instance%20Parameter%20Value 0.0)
    (else
      (LocalVariables|SetFMODEvent "/Game/FMOD/Events/SFX/Objects/MovingPlattform/MovingPlattformOff.MovingPlattformOff")
      (LocalVariables|SetFMODEvent%20Instance%20Parameter%20Value 1.0)))
  (bind _returnvalue (Class|FMODBlueprintStatics|EventInstanceIsValid (Variables|Default|GetFMODEvent%20Instance)))
  (if _returnvalue
    _
    (else
      (bind _returnvalue_2 (Class|FMODBlueprintStatics|PlayEvent2D (LocalVariables|GetFMODEvent)))
      (Variables|Default|SetFMODEvent%20Instance _returnvalue_2)))
  (Class|FMODBlueprintStatics|EventInstanceSetParameter (Variables|Default|GetFMODEvent%20Instance) "PlattformState" (LocalVariables|GetFMODEvent%20Instance%20Parameter%20Value)))

(fn DisablePlayerMovementifTop
  (if (Utilities|Array|IsNotEmpty (Collision|GetOverlappingActors (Variables|Default|GetBox) "/Game/Blueprints/Character/Hero/BP_Hero.BP_Hero_C" :!class /Script/Engine.PrimitiveComponent))
    (Class|BPIHero|DisableMovement(Message) (Game|GetPlayerCharacter 0))
    (Variables|Default|SetHasDisabledPlayerMovement true)))

(fn EnablePlayerMovement
  (if (Variables|Default|GetHasDisabledPlayerMovement)
    (Class|BPIHero|EnableMovement(Message) (Game|GetPlayerCharacter 0))
    (Variables|Default|SetHasDisabledPlayerMovement false)))

(fn GetSpudRespawnMode
  (return "Default"))

(fn OverrideName
  (return ""))

(fn ShouldSkipRestoreTransform
  (return false))

(fn ShouldSkipRestoreVelocity
  (return false))