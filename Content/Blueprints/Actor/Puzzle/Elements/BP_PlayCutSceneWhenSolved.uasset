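; BP_PlayCutSceneWhenSolved is a puzzle actor that plays a cutscene on BeginPlay if its assigned puzzle is the last one solved.
; It asks BP_GameInstance through IsLastPuzzleSolved, then creates and plays a level sequence player for its LevelSequence.
; When the sequence finishes, a bound event sets the player controller's view target back to BP_Hero's FollowCamera.
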(event Custom|ReturnToCamera
  (bind _asbp_hero (Utilities|Casting|CastToBP_Hero (Game|GetPlayerCharacter 0)))
  (Game|Player|SetViewTargetwithBlend (Game|GetPlayerController 0) (Variables|/Script/HeartWeaver.KrakenCharacter|GetFollowCamera _asbp_hero) 0.0 "VTBlend_Linear" 0.0 false))

(event EventBeginPlay
  (CallFunction|GetGameInstance)
  (if (Default|IsLastPuzzleSolved (Variables|Default|GetAs%20BP%20Game%20Instance) (Variables|Default|GetPuzzle))
    (bind _returnvalue (Sequencer|Player|CreateLevelSequencePlayer (Variables|Default|GetLevelSequence) (Utilities|Struct|MakeMovieSceneSequencePlaybackSettings true "(Value=0)" 1.0 0.0 false false false false false false "None" false)))
    (Sequencer|Player|Play _returnvalue :!class /Script/MovieScene.MovieSceneSequencePlayer)
    (EventDispatchers|BindEventtoOnFinished _returnvalue (delegate Custom|ReturnToCamera))))

(fn ConstructionScript)

(fn GetGameInstance
  (bind _asbp_game_instance (Utilities|Casting|CastToBP_GameInstance (Game|GetGameInstance)))
  (Variables|Default|SetAs%20BP%20Game%20Instance _asbp_game_instance))