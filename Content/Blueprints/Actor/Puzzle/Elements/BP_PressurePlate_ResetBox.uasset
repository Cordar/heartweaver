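; Puzzle pressure plate that teleports the boxes in BoxToReset back to their respawn points when the hero or a pushable object steps on it.
; Overlap fires Activated and lowers the button by timeline; it reverses and fires Deactivated once no hero or BP_PushableObject remains.
; Both transitions play the PressurePlateDeactivate sound.
; An async-loaded moving platform reference, HideOnActivatingThisActor, destroys the plate when that platform activates.
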(event OnComponentBeginOverlap(Box)
  (params (OverlappedComponent :type Primitive%20Component%20Object%20Reference) (OtherActor :type Actor%20Object%20Reference) (OtherComp :type Primitive%20Component%20Object%20Reference) (OtherBodyIndex :type Integer) (bFromSweep :type Boolean) (SweepResult :type Hit%20Result%20Structure%20%28by%20ref%29))
  (Utilities|Casting|CastToBP_Hero OtherActor
    (:then
      (Class|KrakenActivableObject|Activate self :!label _label)
      (for _array_element (Variables|Default|GetBoxToReset)
        (Transformation|SetActorLocation _array_element (Transformation|GetActorLocation (Variables|/Game/Blueprints/Actor/Puzzle/Elements/PushableObject/BP_PushableNumbnessBox.BP_PushableNumbnessBox_C|GetRespawnPoint _array_element)) false false)))
    (:CastFailed
      (if (Utilities|DoesObjectImplementInterface OtherActor "/Script/HeartWeaver.KrakenPushableObject")
        (goto _label)))))

(event OnComponentEndOverlap(Box)
  (params (OverlappedComponent :type Primitive%20Component%20Object%20Reference) (OtherActor :type Actor%20Object%20Reference) (OtherComp :type Primitive%20Component%20Object%20Reference) (OtherBodyIndex :type Integer))
  (if (and (Utilities|Array|IsEmpty (Collision|GetOverlappingActors (Variables|Default|GetBox) "/Game/Blueprints/Actor/Puzzle/Elements/PushableObject/BP_PushableObject.BP_PushableObject_C" :!class /Script/Engine.PrimitiveComponent)) (Utilities|Array|IsEmpty (Collision|GetOverlappingActors (Variables|Default|GetBox) "/Game/Blueprints/Character/Hero/BP_Hero.BP_Hero_C" :!class /Script/Engine.PrimitiveComponent)))
    (Class|KrakenActivableObject|Deactivate)))

(event Custom|Destroy
  (Actor|DestroyActor))

(event EventActivate
  (params (Instigator :type Actor%20Object%20Reference))
  (Default|CallActivated Instigator)
  (Class|FMODBlueprintStatics|PlayEventatLocation "/Game/FMOD/Events/SFX/Objects/PressurePlate/PressurePlateDeactivate.PressurePlateDeactivate" (Transformation|GetActorTransform))
  (bind _newtrack_0 (Timeline|Button%20Timeline Play)
    (:Update
      (Transformation|SetRelativeLocation (Variables|Default|GetButton) (Math|Vector|MakeVector 0.0 0.0 (Math|Float|Lerp 0.0 -11.0 _newtrack_0)) false false))))

(event EventDeactivate
  (Class|FMODBlueprintStatics|PlayEventatLocation "/Game/FMOD/Events/SFX/Objects/PressurePlate/PressurePlateDeactivate.PressurePlateDeactivate" (Transformation|GetActorTransform))
  (Default|CallDeactivated)
  (bind _newtrack_0 (Timeline|Button%20Timeline Reverse)
    (:Update
      (Transformation|SetRelativeLocation (Variables|Default|GetButton) (Math|Vector|MakeVector 0.0 0.0 (Math|Float|Lerp 0.0 -11.0 _newtrack_0)) false false))))

(event EventBeginPlay
  (bind _object (Utilities|AsyncLoadAsset (Variables|Default|GetHideOnActivatingThisActor))
    (:Completed
      (bind _asbp_moving_platform (Utilities|Casting|CastToBP_MovingPlatform _object))
      (EventDispatchers|BindEventtoActivated _asbp_moving_platform (delegate Custom|Destroy)))))

(fn ConstructionScript)