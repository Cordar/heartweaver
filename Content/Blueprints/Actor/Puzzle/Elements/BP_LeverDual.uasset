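; BP_LeverDual is a puzzle lever that works as a pair with a linked OtherLever, extending a parent lever's activation and deactivation.
; On activation, if the partner is already active, it clears both levers' deactivation timers and starts a new one using SecondsToDeactivateWhenBothActivated.
; That timer targets only this lever's deactivation, as the call to deactivate the partner is disconnected and never runs.
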(event Custom|ActivatedEvent
  (params (Instigator :type Actor%20Object%20Reference))
  (bind _otherlever (Variables|Default|GetOtherLever))
  (|CallParentFunction Instigator)
  (Utilities|IsValid _otherlever
    (:Is%20Valid
      (if (Variables|/Game/Blueprints/Actor/Puzzle/Elements/BP_Lever.BP_Lever_C|GetIsActive _otherlever)
        (Utilities|Time|ClearandInvalidateTimerbyHandle (Variables|/Game/Blueprints/Actor/Puzzle/Elements/BP_LeverTemporary.BP_LeverTemporary_C|GetDeactivateTimerHandle _otherlever))
        (Utilities|Time|ClearandInvalidateTimerbyHandle (Variables|Default|GetDeactivateTimerHandle))
        (Utilities|Time|SetTimerbyEvent (delegate EventDeactivate) (Variables|Default|GetSecondsToDeactivateWhenBothActivated))))))

(event EventDeactivate
  (|CallParentFunction))

(fn ConstructionScript
  (|CallParentFunction))