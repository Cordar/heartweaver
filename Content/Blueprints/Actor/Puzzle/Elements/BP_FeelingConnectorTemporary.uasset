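; BP_FeelingConnectorTemporary is a puzzle connector that switches on its linked Activable for a limited time.
; Activate sends the activate message and starts a one-shot timer of SecondsToDeactivate, which fires Deactivate to send the deactivate message.
; An IsActivated flag ignores repeat activations while active, so they do not restart the countdown.
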(event EventDeactivate
  (Class|KrakenActivableObject|Deactivate(Message) (Variables|Default|GetActivable))
  (Variables|Default|SetIs%20Activated false))

(event EventActivate
  (if (not (Variables|Default|GetIs%20Activated))
    (Class|KrakenActivableObject|Activate(Message) (Variables|Default|GetActivable))
    (Variables|Default|SetIs%20Activated true)
    (Utilities|Time|SetTimerbyEvent (delegate EventDeactivate) (Variables|Default|GetSeconds%20To%20Deactivate))))

(fn ConstructionScript
  (|CallParentFunction))