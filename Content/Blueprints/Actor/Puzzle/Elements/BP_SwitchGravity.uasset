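; Puzzle ramp that lets the Kraken character walk on walls by changing its gravity direction.
; While the character overlaps the box, Tick sets gravity opposite the nearest child arrow's forward vector and a GameplayEffect disables jumping.
; Exiting snaps gravity to the nearer end arrow and restores jumping.
; An optional puzzle link hides it until solved, revealing it with Niagara and a scale-up timeline if that puzzle was solved last.
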(event OnComponentBeginOverlap(Box)
  (params (OverlappedComponent :type Primitive%20Component%20Object%20Reference) (OtherActor :type Actor%20Object%20Reference) (OtherComp :type Primitive%20Component%20Object%20Reference) (OtherBodyIndex :type Integer) (bFromSweep :type Boolean) (SweepResult :type Hit%20Result%20Structure%20%28by%20ref%29))
  (if (Variables|Default|GetIsActive)
    (bind _askraken_character (Utilities|Casting|CastToKrakenCharacter OtherActor))
    (Variables|Default|SetCurrentCharacter _askraken_character)
    (Class|FMODBlueprintStatics|PlayEvent2D "/Game/FMOD/Events/SFX/Player/Locomotion/Misc/WallWalk.WallWalk")
    (bind _returnvalue (GameplayEffects|ApplyGameplayEffectToSelf :self (Ability|GetAbilitySystemComponent (Variables|Default|GetCurrentCharacter)) :GameplayEffectClass "/Game/Blueprints/Character/Hero/GameplayEffect/GE_DisableJump.GE_DisableJump_C"))
    (Variables|Default|SetDisableJump _returnvalue)))

(event OnComponentEndOverlap(Box)
  (params (OverlappedComponent :type Primitive%20Component%20Object%20Reference) (OtherActor :type Actor%20Object%20Reference) (OtherComp :type Primitive%20Component%20Object%20Reference) (OtherBodyIndex :type Integer))
  (bind _arrowcomponents (Variables|Default|GetArrowComponents))
  (bind _returnvalue (Utilities|Array|Length _arrowcomponents))
  (bind _output (Utilities|Array|Get(acopy) _arrowcomponents))
  (bind _returnvalue_2 (- _returnvalue 1))
  (bind _output_2 (Utilities|Array|Get(acopy) _arrowcomponents _returnvalue_2))
  (if (Variables|Default|GetIsActive)
    (Utilities|Casting|CastToKrakenCharacter OtherActor)
    (Utilities|IsValid (Variables|Default|GetCurrentCharacter)
      (:Is%20Valid
        (Utilities|FlowControl|Sequence
          (:then_0
            (if (> (Math|Vector|Distance(Vector) (Transformation|GetActorLocation (Variables|Default|GetCurrentCharacter)) (Transformation|GetWorldLocation _output)) (Math|Vector|Distance(Vector) (Transformation|GetActorLocation (Variables|Default|GetCurrentCharacter)) (Transformation|GetWorldLocation _output_2)))
              (Class|CharacterMovementComponent|SetGravityDirection (Variables|/Script/HeartWeaver.KrakenCharacter|GetKrakenCharacterMovementComponent (Variables|Default|GetCurrentCharacter)) (Math|Vector|Normalize (Math|Vector|NegateVector (Math|Vector|GetForwardVector _output_2))))
              (else
                (Class|CharacterMovementComponent|SetGravityDirection (Variables|/Script/HeartWeaver.KrakenCharacter|GetKrakenCharacterMovementComponent (Variables|Default|GetCurrentCharacter)) (Math|Vector|Normalize (Math|Vector|NegateVector (Math|Vector|GetForwardVector _output)))))))
          (:then_1
            (Utilities|IsValid (Variables|Default|GetCurrentCharacter)
              (:Is%20Valid
                (GameplayEffects|RemoveActiveGameplayEffect (Ability|GetAbilitySystemComponent (Variables|Default|GetCurrentCharacter)) (Variables|Default|GetDisableJump) -1))
              (:Is%20Not%20Valid
                _))
            (Variables|Default|SetCurrentCharacter 0)))))))

(event Custom|AppearMagically
  (bind _returnvalue (AddComponent|AddNiagaraComponent false))
  (Class|NiagaraComponent|SetAutoDestroy _returnvalue true)
  (Class|NiagaraComponent|SetAsset _returnvalue "/Game/Assets/VFX/NS_AppearGravitySwitch.NS_AppearGravitySwitch" true)
  (Variables|Default|SetInitialScale (Transformation|GetActorScale3D))
  (Transformation|SetActorScale3D "0, 0, 0")
  (Rendering|SetActorHiddenInGame false)
  (bind _newtrack_0 (Timeline|Timeline Play)
    (:Update
      (Transformation|SetActorScale3D (Math|Vector|Lerp(Vector) "0, 0, 0" (Variables|Default|GetInitialScale) _newtrack_0)))
    (:Finished
      (Variables|Default|SetIsActive true))))

(event Custom|OldMethod
  ;[0.01096 0.01161 0.0137] Método antiguo
  (if (Variables|Default|GetIsActive)
    (bind _currentcharacter (Variables|Default|GetCurrentCharacter)
      (:then
        (Variables|Default|SetDistanceToCharacter 5e+07)
        (for _array_element (Variables|Default|GetArrowComponents)
          (if (<= (Math|Vector|Distance(Vector) (Transformation|GetWorldLocation _array_element) (Transformation|GetActorLocation _currentcharacter)) (Variables|Default|GetDistanceToCharacter))
            (Variables|Default|SetNormalForGravity (Math|Vector|NegateVector (Math|Vector|GetForwardVector _array_element)))
            (Variables|Default|SetDistanceToCharacter (Math|Vector|Distance(Vector) (Transformation|GetWorldLocation _array_element) (Transformation|GetActorLocation _currentcharacter)))))
        (Class|CharacterMovementComponent|SetGravityDirection (Variables|/Script/HeartWeaver.KrakenCharacter|GetKrakenCharacterMovementComponent (Variables|Default|GetCurrentCharacter)) (Math|Vector|Normalize (Variables|Default|GetNormalForGravity))))
      (:else))))

(event EventBeginPlay
  (Utilities|FlowControl|Sequence
    (:then_0
      (Utilities|Array|Clear (Variables|Default|GetArrowComponents))
      (for _array_element (Components|GetChildrenComponents (Variables|Default|GetStaticMesh) true)
        (bind _asarrow_component (Utilities|Casting|CastToArrowComponent _array_element))
        (Utilities|Array|Add (Variables|Default|GetArrowComponents) _asarrow_component))
      (if (Utilities|Enum|NotEqual(Enum) (Variables|Default|GetPuzzleSolved) "NewEnumerator9")
        (CallFunction|GetGameInstance)
        (bind _issolved (Default|IsPuzzleSolved (Variables|Default|GetAs%20BP%20Game%20Instance) (Variables|Default|GetPuzzleSolved)))
        (if _issolved
          (if (Default|IsLastPuzzleSolved (Variables|Default|GetAs%20BP%20Game%20Instance) (Variables|Default|GetPuzzleSolved))
            (CallFunction|AppearMagically)
            (Class|FMODBlueprintStatics|PlayEvent2D "/Game/FMOD/Events/SFX/Objects/Ramp/RampMagicallyAppear.RampMagicallyAppear")
            (else
              (Variables|Default|SetIsActive true)))
          (else
            (Rendering|SetActorHiddenInGame true)))
        (else
          (Variables|Default|SetIsActive true))))))

(event EventTick
  (params (DeltaSeconds :type Float%20%28single-precision%29))
  (CallFunction|OldMethod))

(fn ConstructionScript)

(fn GetGameInstance
  (bind _asbp_game_instance (Utilities|Casting|CastToBP_GameInstance (Game|GetGameInstance)))
  (Variables|Default|SetAs%20BP%20Game%20Instance _asbp_game_instance))