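; BP_NPC is a one-shot dialogue actor that runs a SUDS script between the player and itself.
; Activation, optionally triggered by BP_Hero entering its box, builds the dialogue widget with two character sub-widgets and switches input to UI.
; As a dialogue participant it pushes each speaker line and any multiple choices to the widget.
; It destroys itself when dialogue ends or its linked puzzle entrance is solved.
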(event OnComponentBeginOverlap(Box)
  (params (OverlappedComponent :type Primitive%20Component%20Object%20Reference) (OtherActor :type Actor%20Object%20Reference) (OtherComp :type Primitive%20Component%20Object%20Reference) (OtherBodyIndex :type Integer) (bFromSweep :type Boolean) (SweepResult :type Hit%20Result%20Structure%20%28by%20ref%29))
  (bind _asbp_hero (Utilities|Casting|CastToBP_Hero OtherActor))
  (if (Variables|Default|GetStartOnOverlap)
    (Class|KrakenActivableObject|Activate _asbp_hero)))

(event Custom|CustomEvent
  (Actor|DestroyActor))

(event EventBeginPlay
  (bind _puzzleentrance (Variables|Default|GetPuzzleEntrance))
  (Utilities|IsValid _puzzleentrance
    (:Is%20Valid
      (EventDispatchers|BindEventtoOnPuzzleSolved _puzzleentrance (delegate Custom|CustomEvent)))))

(event EventDeactivate
  (bind _returnvalue (Game|GetPlayerController 0))
  (Widget|RemovefromParent (Variables|Default|GetDialogueWidget))
  (Variables|/Script/Engine.PlayerController|SetbShowMouseCursor _returnvalue false)
  (Input|SetInputModeGameOnly _returnvalue false)
  (Actor|DestroyActor))

(event EventOnDialogueSpeakerLine
  (params (Dialogue :type SUDS%20Dialogue%20Object%20Reference))
  (CallFunction|SetWidgetText Dialogue))

(event EventOnDialogueFinished
  (params (Dialogue :type SUDS%20Dialogue%20Object%20Reference))
  (CallFunction|Deactivate))

(event EventActivate
  (params (Instigator :type Actor%20Object%20Reference))
  (bind _returnvalue (Game|GetPlayerController 0))
  (bind _returnvalue_2 (UserInterface|CreateWidget "/Game/Blueprints/UI/Widget/Dialogue/WBP_DialogueWithCharacters.WBP_DialogueWithCharacters_C" (Game|GetPlayerController 0)))
  (Variables|Default|SetDialogueWidget _returnvalue_2)
  (bind _returnvalue_3 (UserInterface|CreateWidget (Variables|Default|GetMainCharacterWidget) (Game|GetPlayerController 0)))
  (Widget|Panel|AddChild (Variables|/Game/Blueprints/UI/Widget/Dialogue/WBP_DialogueWithCharacters.WBP_DialogueWithCharacters_C|GetMainCharacter (Variables|Default|GetDialogueWidget)) _returnvalue_3)
  (bind _returnvalue_4 (UserInterface|CreateWidget (Variables|Default|GetOtherCharacterWidget) (Game|GetPlayerController 0)))
  (Widget|Panel|AddChild (Variables|/Game/Blueprints/UI/Widget/Dialogue/WBP_DialogueWithCharacters.WBP_DialogueWithCharacters_C|GetOtherCharacter (Variables|Default|GetDialogueWidget)) _returnvalue_4)
  (bind _returnvalue_5 (Class|SUDSLibrary|CreateDialoguewithParticipants self (Variables|Default|GetSUDSScript) (Utilities|Array|MakeArray (Game|GetPlayerCharacter 0) self) false "None"))
  (Utilities|IsValid _returnvalue_5
    (:Is%20Valid
      (bind _output_get (Variables|Default|SetSUDSDialogue _returnvalue_5))
      (Variables|/Game/Blueprints/UI/Widget/Dialogue/WBP_DialogueWithCharacters.WBP_DialogueWithCharacters_C|SetSUDSDialogue (Variables|Default|GetDialogueWidget) _output_get)
      (UserInterface|Viewport|AddtoViewport (Variables|Default|GetDialogueWidget) 0)
      (Variables|/Script/Engine.PlayerController|SetbShowMouseCursor _returnvalue true)
      (Input|SetInputModeUIOnly _returnvalue (Variables|Default|GetDialogueWidget) "DoNotLock" false)
      (Class|SUDSDialogue|Start (Variables|Default|GetSUDSDialogue) "None"))
    (:Is%20Not%20Valid
      (CallFunction|Deactivate))))

(fn ConstructionScript)

(fn SetWidgetText
  (params (Dialogue :type SUDS%20Dialogue%20Object%20Reference))
  (bind _returnvalue (Class|SUDSDialogue|GetNumberOfChoices Dialogue))
  (Default|SetLineText (Variables|Default|GetDialogueWidget) (Class|SUDSDialogue|GetText Dialogue))
  (Default|SetCharacter (Variables|Default|GetDialogueWidget) (Class|SUDSDialogue|GetSpeakerDisplayName Dialogue))
  (LocalVariables|SetNumberOfChoices _returnvalue)
  (if (> _returnvalue 1)
    (Default|ShowChoiceWidget (Variables|Default|GetDialogueWidget))
    (for _index (range 0 (- (LocalVariables|GetNumberOfChoices) 1))
      (bind _returnvalue_2 (Class|SUDSDialogue|GetChoiceText Dialogue _index))
      (Default|SetChoice (Variables|Default|GetDialogueWidget) _index _returnvalue_2))
    (else
      (Default|HideChoiceWidget (Variables|Default|GetDialogueWidget)))))

(fn GetDialogueParticipantPriority
  (return 0))