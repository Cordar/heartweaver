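; Interactable dialogue actor that runs a SUDS script between itself and the player character when activated.
; Activate creates a WBP_DialogueSimple widget and the dialogue, passes an IsFirstTime flag into the script so it can tell repeat visits apart, then starts both.
; As a dialogue participant, it pushes each line's text and speaker name to the widget and stops the UI when the dialogue finishes.
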(event EventActivate
  (bind _returnvalue (UserInterface|CreateWidget "/Game/Blueprints/UI/Subwidget/Dialogue/WBP_DialogueSimple.WBP_DialogueSimple_C" (Game|GetPlayerController 0)))
  (Variables|Default|SetDialogueWidget _returnvalue)
  (bind _returnvalue_2 (Class|SUDSLibrary|CreateDialoguewithParticipants self (Variables|Default|GetSUDSScript) (Utilities|Array|MakeArray (Game|GetPlayerCharacter 0) self) false "None"))
  (bind _output_get (Variables|Default|SetSUDSDialogue _returnvalue_2))
  (Variables|/Game/Blueprints/UI/Subwidget/Dialogue/WBP_DialogueSimple.WBP_DialogueSimple_C|SetSUDSDialogue (Variables|Default|GetDialogueWidget) _output_get)
  (Class|SUDSDialogue|SetVariableBoolean (Variables|Default|GetSUDSDialogue) "IsFirstTime" (Variables|Default|GetIsFirstTime))
  (Variables|Default|SetIsFirstTime false)
  (Class|SUDSDialogue|Start (Variables|Default|GetSUDSDialogue) "None")
  (CallFunction|StartUI (Variables|Default|GetDialogueWidget)))

(event EventOnDialogueSpeakerLine
  (params (Dialogue :type SUDS%20Dialogue%20Object%20Reference))
  (CallFunction|SetWidgetData Dialogue))

(event EventOnDialogueFinished
  (params (Dialogue :type SUDS%20Dialogue%20Object%20Reference))
  (CallFunction|StopUI (Variables|Default|GetDialogueWidget)))

(fn ConstructionScript)

(fn SetWidgetData
  (params (Dialogue :type SUDS%20Dialogue%20Object%20Reference))
  (LocalVariables|SetLoc_Dialogue Dialogue)
  (Default|SetMessage (Variables|Default|GetDialogueWidget) (Class|SUDSDialogue|GetText (LocalVariables|GetLoc_Dialogue)))
  (Default|SetName (Variables|Default|GetDialogueWidget) (Class|SUDSDialogue|GetSpeakerDisplayName (LocalVariables|GetLoc_Dialogue))))

(fn GetDialogueParticipantPriority
  (return 0))