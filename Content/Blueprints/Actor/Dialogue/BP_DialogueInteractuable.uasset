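; Interactable actor that BP_Hero targets by proximity to play a SUDS dialogue in a simple widget.
; Activation picks a first-time or repeat level sequence, passes IsFirstTime to the script and starts dialogue immediately if flagged or no sequence exists.
; Deactivation closes the UI and jumps the cutscene to its end.
; Optional corruption overlays a slightly enlarged BP_CorruptedMesh copy, blocking interaction until cleansed, then restores targeting and custom depth.
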(event OnComponentBeginOverlap(Sphere)
  (params (OverlappedComponent :type Primitive%20Component%20Object%20Reference) (OtherActor :type Actor%20Object%20Reference) (OtherComp :type Primitive%20Component%20Object%20Reference) (OtherBodyIndex :type Integer) (bFromSweep :type Boolean) (SweepResult :type Hit%20Result%20Structure%20%28by%20ref%29))
  (bind _asbp_hero (Utilities|Casting|CastToBP_Hero OtherActor))
  (if (and (Variables|Default|GetIsCorrupted) (Variables|Default|GetShouldBeCorrupted))
    (Variables|Dialogue|SetShouldShowWidgetWhenCleansed true)
    (else
      (Class|KrakenInteractableActor|SetasTarget _asbp_hero))))

(event OnComponentEndOverlap(Sphere)
  (params (OverlappedComponent :type Primitive%20Component%20Object%20Reference) (OtherActor :type Actor%20Object%20Reference) (OtherComp :type Primitive%20Component%20Object%20Reference) (OtherBodyIndex :type Integer))
  (bind _asbp_hero (Utilities|Casting|CastToBP_Hero OtherActor))
  (if (and (Variables|Default|GetIsCorrupted) (Variables|Default|GetShouldBeCorrupted))
    (Variables|Dialogue|SetShouldShowWidgetWhenCleansed false)
    (else
      (Class|KrakenInteractableActor|UnsetasTarget _asbp_hero))))

(event Custom|ContinueDialogue
  (Class|SUDSDialogue|Continue (Variables|Default|GetSUDSDialogue)))

(event EventDeactivate
  (bind _cutscene (Variables|Dialogue|GetCutscene))
  (bind _sequenceplayer (Variables|/Script/LevelSequence.LevelSequenceActor|GetSequencePlayer _cutscene))
  (bind _returnvalue (Class|MovieSceneSequencePlayer|GetEndTime _sequenceplayer))
  (|CallParentFunction)
  (CallFunction|StopUI (Variables|Default|GetDialogueWidget))
  (Utilities|IsValid _cutscene
    (:Is%20Valid
      (Components|Timeline|SetPlaybackPosition _sequenceplayer (Utilities|Struct|MakeMovieSceneSequencePlaybackParams (Utilities|Struct|MakeFrameTime (.frame _returnvalue) (.subframe _returnvalue)) 0.0 "" "(Hours=0,Minutes=0,Seconds=0,Frames=0,bDropFrameFormat=False)" "Frame" "Play" false)))))

(event EventBeginPlay
  (CallFunction|GetHUD)
  (if (Variables|Default|GetShouldBeCorrupted)
    (if (Variables|Default|GetIsCorrupted)
      (CallFunction|SetCorruption)
      (EventDispatchers|BindEventtoFinishedActivation (Variables|Default|GetAs%20BP%20Corrupted%20Mesh) (EventDispatchers|CreateEvent :!event CleanseCorruption)))))

(event EventActivate
  (params (Instigator :type Actor%20Object%20Reference))
  (if (not (and (Variables|Default|GetIsCorrupted) (Variables|Default|GetShouldBeCorrupted)))
    (|CallParentFunction Instigator)
    (Utilities|IsValid (Variables|Default|GetDialogueWidget)
      (:Is%20Valid
        _)
      (:Is%20Not%20Valid
        (bind _returnvalue (UserInterface|CreateWidget "/Game/Blueprints/UI/Widget/Dialogue/WBP_DialogueSimple.WBP_DialogueSimple_C" (Game|GetPlayerController 0)))
        (Variables|Default|SetDialogueWidget _returnvalue)))
    (bind _returnvalue_2 (Class|SUDSLibrary|CreateDialoguewithParticipants self (Variables|Dialogue|GetSUDSScript) (Utilities|Array|MakeArray (Game|GetPlayerCharacter 0) self) false "None"))
    (Utilities|IsValid _returnvalue_2
      (:Is%20Valid
        (bind _output_get (Variables|Default|SetSUDSDialogue _returnvalue_2))
        (Variables|/Game/Blueprints/UI/Widget/Dialogue/WBP_DialogueSimple.WBP_DialogueSimple_C|SetSUDSDialogue (Variables|Default|GetDialogueWidget) _output_get)
        (Class|SUDSDialogue|SetVariableBoolean (Variables|Default|GetSUDSDialogue) "IsFirstTime" (Variables|Default|GetIsFirstTime))
        (if (Variables|Default|GetIsFirstTime)
          (Variables|Dialogue|SetLevelSequenceToPlay (Variables|Dialogue|GetLevel%20Sequence%20First%20Time))
          (Variables|Default|SetIsFirstTime false)
          (else
            (Variables|Dialogue|SetLevelSequenceToPlay (Variables|Dialogue|GetLevel%20Sequence%20Not%20First%20Time))))
        (Utilities|IsValid (Variables|Dialogue|GetLevelSequenceToPlay)
          (:Is%20Valid
            (CallFunction|PlayLevelSequence))
          (:Is%20Not%20Valid
            (Variables|Dialogue|SetCutscene 0)))
        (if (or (Variables|Dialogue|GetShouldStartWhenActivate) (not (Utilities|IsValid (Variables|Dialogue|GetLevelSequenceToPlay))))
          (CallFunction|StartDialogue)))
      (:Is%20Not%20Valid
        (Class|KrakenActivableObject|Deactivate)))))

(event EventOnDialogueSpeakerLine
  (params (Dialogue :type SUDS%20Dialogue%20Object%20Reference))
  (CallFunction|SetWidgetData Dialogue))

(event EventOnDialogueFinished
  (params (Dialogue :type SUDS%20Dialogue%20Object%20Reference))
  (Class|KrakenActivableObject|Deactivate))

(fn ConstructionScript)

(fn SetWidgetData
  (params (Dialogue :type SUDS%20Dialogue%20Object%20Reference))
  (LocalVariables|SetLoc_Dialogue Dialogue)
  (Default|SetMessage (Variables|Default|GetDialogueWidget) (Class|SUDSDialogue|GetText (LocalVariables|GetLoc_Dialogue)))
  (Default|SetName (Variables|Default|GetDialogueWidget) (Class|SUDSDialogue|GetSpeakerDisplayName (LocalVariables|GetLoc_Dialogue))))

(fn StartDialogue
  (Class|SUDSDialogue|Start (Variables|Default|GetSUDSDialogue) "None")
  (CallFunction|StartUI (Variables|Default|GetDialogueWidget) (Variables|Default|GetAs%20Kraken%20HUD)))

(fn GetHUD
  (bind _askraken_hud (Utilities|Casting|CastToKrakenHUD (HUD|GetHUD (Game|GetPlayerController 0))))
  (Variables|Default|SetAs%20Kraken%20HUD _askraken_hud))

(fn SetCorruption
  (bind _asbp_corrupted_mesh (Utilities|Casting|CastToBP_CorruptedMesh (Variables|/Script/Engine.ChildActorComponent|GetChildActor (Variables|Default|GetChildActor))))
  (bind _output_get (Variables|Default|SetAs%20BP%20Corrupted%20Mesh _asbp_corrupted_mesh))
  (Components|StaticMesh|SetStaticMesh (Variables|/Game/Blueprints/Actor/Connectable/BP_CorruptedMesh.BP_CorruptedMesh_C|GetStaticMeshComponent _output_get) (Variables|/Script/Engine.StaticMeshComponent|GetStaticMesh (Variables|Default|GetStaticMesh)))
  (Transformation|SetRelativeScale3D (Variables|/Game/Blueprints/Actor/Connectable/BP_CorruptedMesh.BP_CorruptedMesh_C|GetStaticMeshComponent _output_get) "1.010000,1.010000,1.010000"))

(fn CleanseCorruption
  (Variables|Default|SetIsCorrupted false)
  (if (Variables|Dialogue|GetShouldShowWidgetWhenCleansed)
    (CallFunction|SetasTargetifHero (Game|GetPlayerCharacter 0))
    (Utilities|Time|SetTimerbyFunctionName 0 "SetRenderPass" 1.0)
    (else
      (Utilities|Time|SetTimerbyFunctionName 0 "SetRenderPass" 1.0))))

(fn SetRenderPass
  (Rendering|SetRenderCustomDepth (Variables|Default|GetStaticMesh) true))

(fn PlayLevelSequence
  (Class|BPIHero|DeactivatePulse(Message) (Game|GetPlayerCharacter 0))
  (bind (_outactor _returnvalue) (Sequencer|Player|CreateLevelSequencePlayer (Variables|Dialogue|GetLevelSequenceToPlay) (Utilities|Struct|MakeMovieSceneSequencePlaybackSettings true "(Value=0)" 1.0 0.0 false false false true)))
  (Variables|Dialogue|SetCutscene _outactor)
  (Sequencer|Player|Play _returnvalue :!class /Script/MovieScene.MovieSceneSequencePlayer))

(fn GetDialogueParticipantPriority
  (return 0))

(fn GetSpudRespawnMode
  (return "Default"))

(fn OverrideName
  (return ""))

(fn ShouldSkipRestoreTransform
  (return false))

(fn ShouldSkipRestoreVelocity
  (return false))