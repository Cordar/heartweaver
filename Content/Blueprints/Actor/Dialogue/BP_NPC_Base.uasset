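; BP_NPC_Base is a base NPC actor that runs SUDS dialogue conversations with the player.
; On activation it builds a dialogue widget with portrait widgets for both characters, starts a SUDS dialogue with player and NPC as participants, shows the cursor, switches to UI-only input and pauses the game.
; Speaker line events push text to the widget; finishing removes it, restores game input and unpauses.
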(event EventActivate
  (params (Instigator :type Actor%20Object%20Reference))
  (bind _returnvalue (Game|GetPlayerController 0))
  (bind _returnvalue_2 (UserInterface|CreateWidget "/Game/Blueprints/UI/Widget/Dialogue/WBP_DialogueWithCharacters.WBP_DialogueWithCharacters_C" (Game|GetPlayerController 0)))
  (Variables|Default|SetDialogueWidget _returnvalue_2)
  (bind _returnvalue_3 (UserInterface|CreateWidget (Variables|Default|GetMainCharacterWidget) (Game|GetPlayerController 0)))
  (Widget|Panel|AddChild (Variables|/Game/Blueprints/UI/Widget/Dialogue/WBP_DialogueWithCharacters.WBP_DialogueWithCharacters_C|GetMainCharacter (Variables|Default|GetDialogueWidget)) _returnvalue_3)
  (bind _returnvalue_4 (UserInterface|CreateWidget (Variables|Default|GetOtherCharacterWidget) (Game|GetPlayerController 0)))
  (Widget|Panel|AddChild (Variables|/Game/Blueprints/UI/Widget/Dialogue/WBP_DialogueWithCharacters.WBP_DialogueWithCharacters_C|GetOtherCharacter (Variables|Default|GetDialogueWidget)) _returnvalue_4)
  (bind _returnvalue_5 (Class|SUDSLibrary|CreateDialoguewithParticipants self (Variables|Default|GetSUDSScript) (Utilities|Array|MakeArray (Game|GetPlayerCharacter 0) self) true "None"))
  (bind _output_get (Variables|Default|SetSUDSDialogue _returnvalue_5))
  (Variables|/Game/Blueprints/UI/Widget/Dialogue/WBP_DialogueWithCharacters.WBP_DialogueWithCharacters_C|SetSUDSDialogue (Variables|Default|GetDialogueWidget) _output_get)
  (UserInterface|Viewport|AddtoViewport (Variables|Default|GetDialogueWidget) 0)
  (Variables|/Script/Engine.PlayerController|SetbShowMouseCursor _returnvalue true)
  (Input|SetInputModeUIOnly _returnvalue (Variables|Default|GetDialogueWidget) "DoNotLock" false)
  (Game|SetGamePaused true))

(event EventOnDialogueSpeakerLine
  (params (Dialogue :type SUDS%20Dialogue%20Object%20Reference))
  (Default|SetLineText (Variables|Default|GetDialogueWidget) (Class|SUDSDialogue|GetText Dialogue)))

(event EventOnDialogueFinished
  (params (Dialogue :type SUDS%20Dialogue%20Object%20Reference))
  (bind _returnvalue (Game|GetPlayerController 0))
  (Widget|RemovefromParent (Variables|Default|GetDialogueWidget))
  (Variables|/Script/Engine.PlayerController|SetbShowMouseCursor _returnvalue false)
  (Input|SetInputModeGameOnly _returnvalue false)
  (Game|SetGamePaused false))

(fn ConstructionScript)

(fn GetDialogueParticipantPriority
  (return 0))