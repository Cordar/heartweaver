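; Player character Blueprint for Ace, handling camera hookup, companion spawning, intro scene, puzzle-level transitions and save/UI widgets.
; Gravity-switch events flip gravity and block movement through a GAS effect until landing or timeout, while Tick pulls gravity toward any target actor.
; A timeline drives the pulse through a material parameter collection.
; Highest and lowest point helpers follow the capsule, lowering the top when crouched to make Ace harder to see.
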(event Custom|OpenLevel
  (Game|OpenLevel(byObjectReference) (stale Custom|EnterPuzzle Level)))

(event Custom|ReenableMovement
  (if (Variables|Default|GetMovementDisabledDueToGravityChange)
    (CallFunction|EnableMovement)
    (Variables|Default|SetMovementDisabledDueToGravityChange false)))

(event Custom|EnterPuzzle
  (params (Level :type World%20Soft%20Object%20Reference))
  (bind _returnvalue (AddComponent|AddNiagaraComponent false))
  (Components|Activation|SetAutoActivate _returnvalue true)
  (Class|NiagaraComponent|SetAutoDestroy _returnvalue true)
  (Class|NiagaraComponent|SetAsset _returnvalue "/Game/Assets/Character/Ace/VFX/Dissolve/NS_AceDissolve.NS_AceDissolve" true)
  (Rendering|SetVisibility (Variables|Character|GetMesh) false false)
  (bind _returnvalue_2 (UserInterface|CreateWidget "/Game/Blueprints/UI/Widget/LoadingScreen/BPW_Loading.BPW_Loading_C" (Game|GetPlayerController 0)))
  (UserInterface|Viewport|AddtoViewport _returnvalue_2 99)
  (Utilities|Time|SetTimerbyEvent (delegate Custom|OpenLevel) 3.0))

(event Custom|Die
  (Animation|Montage|PlayMontage (Variables|Character|GetMesh) "/Game/Assets/Character/Ace/Animation/Montage/AM_Ace_Hit.AM_Ace_Hit"))

(event EventBeginPlay
  (CallFunction|InitVariables)
  (CallFunction|SpawnCompanionifActive)
  (Class|GlobalEventSystemBPLibrary|GESBindTagEventtoDelegate "(TagName=\"Event.Gravity.Switch\")" (EventDispatchers|CreateEvent :!event SwitchGravity))
  (CallFunction|InitFace)
  (EventDispatchers|BindEventtoOnPushShouldEnd (Variables|Default|GetKrakenPushComponent) (EventDispatchers|CreateEvent :!event EndPush))
  (CallFunction|CreateStartWidget)
  (EventDispatchers|BindEventtoPreSaveGame (Subsystems|GetSpudSubsystem) (EventDispatchers|CreateEvent :!event CreateSavingWidget)))

(event EventEnableMovement
  (GameplayEffects|RemoveActiveEffectswithTags (Ability|GetAbilitySystemComponent 0) "(GameplayTags=((TagName=\"Gameplay.MovementStopped\")))"))

(event EventOnMovementModeChanged
  (params (PrevMovementMode :type EMovementMode%20Enum :default "MOVE_None") (NewMovementMode :type EMovementMode%20Enum :default "MOVE_None") (PrevCustomMode :type Byte :default 0) (NewCustomMode :type Byte :default 0))
  (if (Math|Boolean|ANDBoolean (Utilities|Enum|NotEqual(Enum) PrevMovementMode "MOVE_Walking") (Utilities|Enum|Equal(Enum) NewMovementMode "MOVE_Walking") (Variables|Default|GetMovementDisabledDueToGravityChange))
    (Variables|Default|SetMovementDisabledDueToGravityChange false)
    (CallFunction|EnableMovement)))

(event EventDisableMovement
  (GameplayEffects|ApplyGameplayEffectToSelf :self (Ability|GetAbilitySystemComponent 0) :GameplayEffectClass "/Game/Blueprints/Character/Hero/GameplayEffect/GE_DisableMovement.GE_DisableMovement_C"))

(event EventActivatePulse
  (bind _returnvalue (Transformation|GetActorLocation))
  (Class|FMODBlueprintStatics|PlayEvent2D)
  (Components|Timeline|SetPlayRate (Variables|Default|GetPulse) 1.0)
  (bind _newtrack_0 (Timeline|Pulse Play)
    (:Update
      (Rendering|Material|SetScalarParameterValue "/Game/Blueprints/VFX/Pulse/MPC_Pulse.MPC_Pulse" "Radius" _newtrack_0 :!class /Script/Engine.KismetMaterialLibrary)
      (Rendering|Material|SetVectorParameterValue "/Game/Blueprints/VFX/Pulse/MPC_Pulse.MPC_Pulse" "PlayerPosition" (Utilities|Struct|MakeLinearColor (.x _returnvalue) (.y _returnvalue) (.z _returnvalue) 1.0) :!class /Script/Engine.KismetMaterialLibrary))))

(event EventPrepareIntroScene
  (Utilities|Time|SetGlobalTimeDilation 0.5)
  (Variables|/Script/Engine.Actor|SetCustomTimeDilation (Variables|Default|GetFollowCamera) 3.0)
  (CallFunction|DisableMovement)
  (Utilities|FlowControl|Delay 3.0)
  (bind _returnvalue (UserInterface|CreateWidget "/Game/Blueprints/UI/Widget/Effect/WBP_UI_FeelEffect.WBP_UI_FeelEffect_C" (Game|GetPlayerController 0)))
  (Variables|Default|SetIntroSceneWidget _returnvalue)
  (UserInterface|Viewport|AddtoViewport _returnvalue 0))

(event EventSetLocation
  (bind _as_bp_game_instance (Variables|Default|GetAs%20BP%20Game%20Instance))
  (Utilities|IsValid _as_bp_game_instance
    (:Is%20Valid
      _)
    (:Is%20Not%20Valid
      (CallFunction|InitVariables)))
  (Transformation|SetActorLocation (Variables|/Game/Blueprints/Game/BP_GameInstance.BP_GameInstance_C|GetPlayerLocation _as_bp_game_instance) false false))

(event EventDeactivatePulse
  (bind _returnvalue (Transformation|GetActorLocation))
  (Class|FMODBlueprintStatics|PlayEvent2D)
  (Components|Timeline|SetPlayRate (Variables|Default|GetPulse) 2.0)
  (bind _newtrack_0 (Timeline|Pulse Reverse)
    (:Update
      (Rendering|Material|SetScalarParameterValue "/Game/Blueprints/VFX/Pulse/MPC_Pulse.MPC_Pulse" "Radius" _newtrack_0 :!class /Script/Engine.KismetMaterialLibrary)
      (Rendering|Material|SetVectorParameterValue "/Game/Blueprints/VFX/Pulse/MPC_Pulse.MPC_Pulse" "PlayerPosition" (Utilities|Struct|MakeLinearColor (.x _returnvalue) (.y _returnvalue) (.z _returnvalue) 1.0) :!class /Script/Engine.KismetMaterialLibrary))))

(event EventPossessed
  (params (NewController :type Controller%20Object%20Reference))
  (CallFunction|ActivateCamera)
  (Utilities|FlowControl|Delay 0.1)
  (bind _asbp_tracking_camera (Utilities|Casting|CastToBP_TrackingCamera (Variables|Default|GetFollowCamera)))
  (Default|FindTrigger _asbp_tracking_camera))

(event EventTick
  (params (DeltaSeconds :type Float%20%28single-precision%29))
  (bind _targetgravityactor (Variables|Default|GetTargetGravityActor)
    (:then
      (Class|CharacterMovementComponent|SetGravityDirection (Variables|Character|GetCharacterMovement) (Math|Vector|Normalize (- (Transformation|GetActorLocation _targetgravityactor) (Transformation|GetActorLocation)))))
    (:else)))

(event EventEndPlay
  (params (EndPlayReason :type EEndPlayReason%20Enum :default "Destroyed"))
  (Class|GlobalEventSystemBPLibrary|GESUnbindTagDelegate "(TagName=\"Event.Gravity.Switch\")" (EventDispatchers|CreateEvent :!event SwitchGravity)))

(event Input|KeyboardEvents|Q
  (params (Key :type Key%20Structure :default "None"))
  (:Pressed
    (bind _returnvalue (Game|GetCurrentLevelName true))
    (if (and (not (Variables|/Game/Blueprints/Game/BP_GameInstance.BP_GameInstance_C|GetIntroScenePlayed (Variables|Default|GetAs%20BP%20Game%20Instance))) (Utilities|Enum|Equal(Enum) _returnvalue "numbness_demo"))
      (Utilities|FlowControl|Delay 1.3)
      (Variables|/Game/Blueprints/Game/BP_GameInstance.BP_GameInstance_C|SetIntroScenePlayed (Variables|Default|GetAs%20BP%20Game%20Instance) true)
      (Widget|RemovefromParent (Variables|Default|GetIntroSceneWidget))
      (CallFunction|EnableMovement)
      (Utilities|FlowControl|Delay 2.0)
      (Utilities|Time|SetGlobalTimeDilation 1.0)
      (Variables|/Script/Engine.Actor|SetCustomTimeDilation (Variables|Default|GetFollowCamera) 1.0))))

(fn ConstructionScript)

(fn MakeLineTrace
  (params (TraceChannel :type ETraceTypeQuery%20Enum :default "TraceTypeQuery1") (ActorsToIgnore :type Array%20of%20Actor%20Object%20References) (DrawDebugType :type EDrawDebugTrace%20Enum :default "None") (TraceDistance :type Float%20%28single-precision%29))
  (bind _returnvalue (Transformation|GetActorLocation))
  (bind (_outhit _returnvalue_2) (Collision|LineTraceByChannel _returnvalue (+ _returnvalue (* (Transformation|GetActorForwardVector) TraceDistance)) TraceChannel false ActorsToIgnore DrawDebugType))
  (return _outhit _returnvalue_2))

(fn ResetWalkSpeed
  (Variables|/Script/Engine.CharacterMovementComponent|SetMaxWalkSpeed (Variables|Default|GetKrakenCharacterMovementComponent) 3e+02))

(fn ActivateCamera
  (bind _returnvalue (Actor|GetActorOfClass "/Game/Blueprints/Camera/BP_TrackingCamera.BP_TrackingCamera_C"))
  (Utilities|IsValid _returnvalue
    (:Is%20Valid
      (Variables|/Game/Blueprints/Camera/BP_TrackingCamera.BP_TrackingCamera_C|SetCharacterToFollow _returnvalue self)
      (Variables|Default|SetFollowCamera _returnvalue))
    (:Is%20Not%20Valid
      (Utilities|Time|SetTimerbyFunctionName 0 "ActivateCamera" 0.1))))

(fn InitFace
  (CallFunction|ChangeHeroFaceExpression "NewEnumerator3"))

(fn InitVariables
  (bind _asbp_game_instance (Utilities|Casting|CastToBP_GameInstance (Game|GetGameInstance)))
  (Variables|Default|SetAs%20BP%20Game%20Instance _asbp_game_instance))

(fn SpawnCompanionifActive
  (bind _returnvalue (Game|GetCurrentLevelName true))
  (if (and (or (Variables|/Game/Blueprints/Game/BP_GameInstance.BP_GameInstance_C|GetIsCompanionActivated (Variables|Default|GetAs%20BP%20Game%20Instance)) (not (Utilities|String|Contains _returnvalue "numbness"))) (not (Utilities|IsValid (Variables|Default|GetBPCompanion))))
    (bind _returnvalue_2 (Game|SpawnActorfromClass "/Game/Blueprints/Character/Companion/BP_Companion.BP_Companion_C" (Math|Transform|MakeTransform (+ (Transformation|GetActorLocation) (Math|Vector|NegateVector (Transformation|GetActorForwardVector))) "0, 0, 0" "1.000000,1.000000,1.000000") "AdjustIfPossibleButAlwaysSpawn" "MultiplyWithRoot" 0 0))
    (Variables|Default|SetBPCompanion _returnvalue_2)))

(fn SwitchGravity
  (params (WildcardProperty :type GES%20Wildcard%20Property%20Structure%20%28by%20ref%29))
  (bind _krakencharactermovementcomponent (Variables|Default|GetKrakenCharacterMovementComponent))
  (bind _gravitydirection (Variables|/Script/Engine.CharacterMovementComponent|GetGravityDirection _krakencharactermovementcomponent))
  (Class|KrakenCharacterMovementComponent|ChangeGravityDirection _krakencharactermovementcomponent (Math|Vector|MakeVector (.x _gravitydirection) (.y _gravitydirection) (* (.z _gravitydirection) -1.0)))
  (CallFunction|DisableMovement)
  (Utilities|Time|SetTimerbyFunctionName 0 "MovementCanBeEnabledWhenTouchingFloorForGravity" 0.5)
  (return))

(fn MovementCanbeEnabledwhenTouchingFloorforGravity
  (Variables|Default|SetMovementDisabledDueToGravityChange true)
  (Utilities|Time|SetTimerbyEvent (EventDispatchers|CreateEvent :!event Custom|ReenableMovement) 2.0))

(fn EndPush
  (Abilities|TryActivateAbilitybyClass (Ability|GetAbilitySystemComponent 0) "/Game/Blueprints/Character/Hero/GameplayAbilities/GA_GrabObject.GA_GrabObject_C" true))

(fn CreateStartWidget
  (bind _returnvalue (UserInterface|CreateWidget "/Game/Blueprints/UI/Widget/LoadingScreen/BPW_StartingMap.BPW_StartingMap_C" (Game|GetPlayerController 0)))
  (UserInterface|Viewport|AddtoViewport _returnvalue -100))

(fn CreateSavingWidget
  (params (SlotName :type String))
  (bind _returnvalue (UserInterface|CreateWidget "/Game/Blueprints/UI/Widget/Effect/WBP_SaveGame.WBP_SaveGame_C" (Game|GetPlayerController 0)))
  (bind _output_get (Variables|Default|SetSaveGameWidget _returnvalue))
  (UserInterface|Viewport|AddtoViewport _output_get 0))

(fn GetHighestPoint
  (if (AI|Components|NavMovement|IsCrouching (Variables|Default|GetKrakenCharacterMovementComponent))
    ;[0.01096 0.01161 0.0137] Si Ace está agachada, queremos que sea más dificil de ver así que le ponemos un punto alto más bajo que la propia cápsula
    (return (Math|Transform|TransformLocation (Transformation|GetActorTransform) (Math|Vector|MakeVector 0.0 0.0 1e+01)))
    (else
      (return (Math|Transform|TransformLocation (Transformation|GetActorTransform) (+ (Math|Vector|MakeVector 0.0 0.0 0.0) (Math|Vector|MakeVector 0.0 0.0 (Components|Capsule|GetUnscaledCapsuleHalfHeight (Variables|Default|GetCapsuleComponent)))))))))

(fn GetLowestPoint
  (return (Math|Transform|TransformLocation (Transformation|GetActorTransform) (- (Math|Vector|MakeVector 0.0 0.0 0.0) (Math|Vector|MakeVector 0.0 0.0 (Components|Capsule|GetUnscaledCapsuleHalfHeight (Variables|Default|GetCapsuleComponent)))))))