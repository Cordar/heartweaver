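; Gameplay ability that lets the hero grab or release grabbable actors and activate interactable ones.
; On activation it tries a grab, then an interact, then ends.
; If the hero can grab, a line trace finds a KrakenGrabableActor to grab; otherwise the hero's current grabbable is released.
; The interact step uses a line trace on a separate channel and sends an activate message to the hit actor.
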(event Ability|EventActivateAbility
  (bind _asbp_hero (Utilities|Casting|CastToBP_Hero (Class|KrakenGameplayAbility|GetKrakenCharacterfromActorInfo)))
  (Variables|Default|SetAs%20BP%20Hero _asbp_hero)
  (Utilities|FlowControl|Sequence
    (:then_0
      (CallFunction|AttemptGrab))
    (:then_1
      (CallFunction|AttemptInteract))
    (:then_2
      (Ability|EndAbility))))

(event Ability|EventOnEndAbility
  (params (bWasCancelled :type Boolean)))

(fn AttemptInteract
  (bind (_outhit _returnvalue) (Default|MakeLineTrace (Variables|Default|GetAs%20BP%20Hero) "TraceTypeQuery5" 0 "None" (Variables|Default|GetTraceDistance)))
  (if _returnvalue
    (Class|KrakenActivableObject|Activate(Message) (.HitActor (Collision|BreakHitResult _outhit)))
    (Ability|EndAbility)))

(fn AttemptGrab
  (bind _as_bp_hero (Variables|Default|GetAs%20BP%20Hero))
  (if (Class|KrakenCharacter|CanGrab (Variables|Default|GetAs%20BP%20Hero))
    (bind (_outhit _returnvalue) (Default|MakeLineTrace (Variables|Default|GetAs%20BP%20Hero) "TraceTypeQuery4" 0 "None" (Variables|Default|GetTraceDistance)))
    (if _returnvalue
      (bind _askraken_grabable_actor (Utilities|Casting|CastToKrakenGrabableActor (.HitActor (Collision|BreakHitResult _outhit))))
      (bind _askraken_character (Utilities|Casting|CastToKrakenCharacter (Ability|GetAvatarActorfromActorInfo)))
      (Class|KrakenGrabableActor|Grab _askraken_grabable_actor _askraken_character))
    (else
      (Class|KrakenGrabableActor|Release (Variables|/Script/HeartWeaver.KrakenCharacter|GetKrakenGrabableActor _as_bp_hero) _as_bp_hero))))