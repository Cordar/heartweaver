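; GA_FeelFear is the hero's fear ability, which temporarily hands player control to a spawned ghost.
; A charge phase swaps the scarf material and sets a charge walk speed, then a release montage plays.
; When the montage completes or is interrupted, it emits a GES tag event and possesses a BP_HeroGhost spawned ahead.
; After FeelTime it emits deactivation and repossesses the hero; ending restores emotion, scarf and a hardcoded speed.
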(event Ability|EventActivateAbility
  (bind _asbp_hero (Utilities|Casting|CastToBP_Hero (Ability|GetAvatarActorfromActorInfo))
    (:then
      (bind _output_get (Variables|Default|SetAs%20BP%20Hero _asbp_hero))
      (Rendering|Material|SetMaterial (Variables|/Script/Engine.Character|GetMesh _output_get) (Variables|Default|GetScarfMaterialIndex) "/Game/Assets/Character/Ace/Material/MI_Character_Ace_Scarf_Fear.MI_Character_Ace_Scarf_Fear")
      (Variables|/Script/Engine.CharacterMovementComponent|SetMaxWalkSpeed (Variables|/Script/HeartWeaver.KrakenCharacter|GetKrakenCharacterMovementComponent (Variables|Default|GetAs%20BP%20Hero)) (Variables|Default|GetChargeMaxWalkSpeed))
      (Class|KrakenCharacter|SetEmotionState (Variables|Default|GetAs%20BP%20Hero) "ES_Fear_Charge")
      (Ability|Tasks|WaitDelay (Variables|Default|GetChargeTime)
        (:OnFinish
          (Class|KrakenCharacter|SetEmotionState (Variables|Default|GetAs%20BP%20Hero) "ES_Fear_Release")
          (Animation|Montage|PlayMontage (Variables|/Script/Engine.Character|GetMesh (Variables|Default|GetAs%20BP%20Hero)) "/Game/Assets/Character/Ace/Animation/Montage/AM_Ace_FearRelease.AM_Ace_FearRelease"
            (:OnCompleted
              _)
            (:OnInterrupted
              _))
          (Class|GlobalEventSystemBPLibrary|GESEmitTagEvent "(TagName=\"Event.Fear.Activated\")" false)
          (bind _returnvalue (Game|SpawnActorfromClass "/Game/Blueprints/Character/HeroGhost/BP_HeroGhost.BP_HeroGhost_C" (Math|Transform|MakeTransform (+ (.location (Transformation|GetActorTransform (Variables|Default|GetAs%20BP%20Hero))) (* (Transformation|GetActorForwardVector (Variables|Default|GetAs%20BP%20Hero)) 1e+02)) (.rotation (Transformation|GetActorTransform (Variables|Default|GetAs%20BP%20Hero))) (.scale (Transformation|GetActorTransform (Variables|Default|GetAs%20BP%20Hero)))) "AdjustIfPossibleButAlwaysSpawn" "MultiplyWithRoot" 0 0))
          (Pawn|Possess (Game|GetPlayerController 0) _returnvalue)
          (Ability|Tasks|WaitDelay (Variables|Default|GetFeelTime)
            (:OnFinish
              (Class|GlobalEventSystemBPLibrary|GESEmitTagEvent "(TagName=\"Event.Fear.Deactivated\")" false)
              (Pawn|Possess (Game|GetPlayerController 0) (Variables|Default|GetAs%20BP%20Hero))
              (Ability|EndAbility))))))
    (:CastFailed
      (Ability|EndAbility))))

(event Ability|EventOnEndAbility
  (params (bWasCancelled :type Boolean))
  (bind _as_bp_hero (Variables|Default|GetAs%20BP%20Hero))
  (Class|KrakenCharacter|SetEmotionState (Variables|Default|GetAs%20BP%20Hero) "ES_Neutral")
  (Rendering|Material|SetMaterial (Variables|/Script/Engine.Character|GetMesh _as_bp_hero) (Variables|Default|GetScarfMaterialIndex) "/Game/Assets/Character/Ace/Material/MI_Character_Ace_Scarf.MI_Character_Ace_Scarf")
  (Variables|/Script/Engine.CharacterMovementComponent|SetMaxWalkSpeed (Variables|/Script/HeartWeaver.KrakenCharacter|GetKrakenCharacterMovementComponent _as_bp_hero) 3.5e+02))