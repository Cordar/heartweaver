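; Gameplay ability for the hero's anger emotion: a charged release that shoves surrounding actors away.
; During the timed charge it overrides walk speed and sets the AngerCharge state, then switches to AngerRelease and plays a montage.
; The montage notify sphere-overlaps nearby actors and applies swept horizontal offsets that grow with distance from the hero, then ends the ability.
; Ending restores the Neutral state and previous walk speed.
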(event Ability|EventActivateAbility
  (bind _returnvalue (Ability|GetAvatarActorfromActorInfo))
  (bind _returnvalue_2 (Class|KrakenGameplayAbility|GetKrakenCharacterfromActorInfo))
  (bind _returnvalue_3 (Class|KrakenGameplayAbility|GetKrakenCharacterfromActorInfo))
  (bind _returnvalue_4 (Transformation|GetActorLocation _returnvalue))
  (bind _krakencharactermovementcomponent (Variables|/Script/HeartWeaver.KrakenCharacter|GetKrakenCharacterMovementComponent _returnvalue_3))
  (Variables|Default|SetOldMax%20Walk%20Speed (Variables|/Script/Engine.CharacterMovementComponent|GetMaxWalkSpeed _krakencharactermovementcomponent))
  (Variables|/Script/Engine.CharacterMovementComponent|SetMaxWalkSpeed _krakencharactermovementcomponent (Variables|Default|GetChargeMaxWalkSpeed))
  (Class|KrakenCharacter|SetEmotionState (Class|KrakenGameplayAbility|GetKrakenCharacterfromActorInfo) "ES_Anger_Charge")
  (Ability|Tasks|WaitDelay (Variables|Default|GetChargeTime)
    (:OnFinish
      (Class|KrakenCharacter|SetEmotionState _returnvalue_2 "ES_Anger_Release")
      (Animation|Montage|PlayMontage (Variables|/Script/Engine.Character|GetMesh _returnvalue_2) "/Game/Assets/Character/Ace/Animation/Montage/AM_Ace_AngerRelease.AM_Ace_AngerRelease"
        (:OnNotifyBegin
          (bind _outactors (Collision|SphereOverlapActors (Transformation|GetActorLocation _returnvalue) (Variables|Default|GetOverlapRadius) (Utilities|Array|MakeArray "ObjectTypeQuery1" "ObjectTypeQuery2" "ObjectTypeQuery3") 0 (Utilities|Array|MakeArray _returnvalue)))
          (for _array_element _outactors
            (Transformation|AddActorWorldOffset _array_element (Math|Vector|MakeVector (.x (* (* (Math|Vector|Distance(Vector) (Transformation|GetActorLocation _array_element) _returnvalue_4) (/ (Variables|Default|GetPushStrength) 1e+03)) (- (Transformation|GetActorLocation _array_element) _returnvalue_4))) (.y (* (* (Math|Vector|Distance(Vector) (Transformation|GetActorLocation _array_element) _returnvalue_4) (/ (Variables|Default|GetPushStrength) 1e+03)) (- (Transformation|GetActorLocation _array_element) _returnvalue_4))) 0.0) true))
          (Ability|EndAbility))))))

(event Ability|EventOnEndAbility
  (params (bWasCancelled :type Boolean))
  (Class|KrakenCharacter|SetEmotionState (Class|KrakenGameplayAbility|GetKrakenCharacterfromActorInfo) "ES_Neutral")
  (Variables|/Script/Engine.CharacterMovementComponent|SetMaxWalkSpeed (Variables|/Script/HeartWeaver.KrakenCharacter|GetKrakenCharacterMovementComponent (Class|KrakenGameplayAbility|GetKrakenCharacterfromActorInfo)) (Variables|Default|GetOldMax%20Walk%20Speed)))