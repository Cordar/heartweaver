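; GA_FeelCancel is a Hero gameplay ability that ends as soon as it activates, with no other logic in its event graph.
; It also holds a GetClosestPushDirection helper, which normalizes an input vector and returns the nearest entry in PossibleDirections by linear distance search.
; Neither event in this graph calls that helper, and the end-ability event is empty.
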(event Ability|EventActivateAbility
  (Ability|EndAbility))

(event Ability|EventOnEndAbility
  (params (bWasCancelled :type Boolean)))

(fn GetClosestPushDirection
  (params (V2 :type Vector))
  (LocalVariables|SetNormalizedInputVector (Math|Vector|Normalize V2))
  (LocalVariables|SetMinDistance 9999.0)
  (for _array_element (Variables|Default|GetPossibleDirections)
    (if (<= (Math|Vector|Distance(Vector) _array_element (LocalVariables|GetNormalizedInputVector)) (LocalVariables|GetMinDistance))
      (LocalVariables|SetChosenDirection_Loc _array_element)
      (LocalVariables|SetMinDistance (Math|Vector|Distance(Vector) _array_element (LocalVariables|GetNormalizedInputVector)))))
  (return (LocalVariables|GetChosenDirection_Loc)))