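; GA_Connect is a hero gameplay ability that emits a pulse to activate nearby connectable actors.
; On activation it fires the Connect gameplay cue and plays the AM_Ace_Pulse montage.
; On montage notify, it activates the character's pulse message, box-overlaps for KrakenConnectableActors within ConnectSize, and calls ActivateMessage on each.
; A Success or Fail cue reports the overlap result, and the ability ends on notify, completion or interruption.
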(event Ability|EventActivateAbility
  (bind _returnvalue (Class|KrakenGameplayAbility|GetKrakenCharacterfromActorInfo))
  (bind _connectsize (Variables|Default|GetConnectSize))
  (GameplayCue|ExecuteGameplayCueOnActor(Burst) (Ability|GetAvatarActorfromActorInfo) "(TagName=\"GameplayCue.Character.Hero.Ability.Ability.Connect\")" (Ability|GameplayCue|MakeGameplayCueParameters :Location (Transformation|GetActorLocation (Ability|GetAvatarActorfromActorInfo))))
  (Animation|Montage|PlayMontage (Variables|/Script/Engine.Character|GetMesh (Class|KrakenGameplayAbility|GetKrakenCharacterfromActorInfo)) "/Game/Assets/Character/Ace/Animation/Montage/AM_Ace_Pulse.AM_Ace_Pulse"
    (:OnCompleted
      (Ability|EndAbility))
    (:OnInterrupted
      (Ability|EndAbility))
    (:OnNotifyBegin
      (Class|BPIHero|ActivatePulse(Message) _returnvalue)
      (bind (_outactors _returnvalue_2) (Collision|BoxOverlapActors (Transformation|GetActorLocation _returnvalue) (Math|Vector|MakeVector _connectsize _connectsize _connectsize) (Utilities|Array|MakeArray "ObjectTypeQuery1" "ObjectTypeQuery2") "/Script/HeartWeaver.KrakenConnectableActor" :!class /Script/Engine.KismetSystemLibrary))
      (if _returnvalue_2
        (GameplayCue|ExecuteGameplayCue :GameplayCueTag "(TagName=\"GameplayCue.Character.Hero.Ability.Ability.Connect.Success\")")
        (for _array_element _outactors
          (Class|KrakenActivableObject|Activate(Message) _array_element))
        (else
          (GameplayCue|ExecuteGameplayCue :GameplayCueTag "(TagName=\"GameplayCue.Character.Hero.Ability.Ability.Connect.Fail\")")))
      (Ability|EndAbility))))

(event Ability|EventOnEndAbility
  (params (bWasCancelled :type Boolean)))