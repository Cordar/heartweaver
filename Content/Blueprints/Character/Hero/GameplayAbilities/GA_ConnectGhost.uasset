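; Gameplay ability that lets the hero ghost "connect" to nearby KrakenConnectableActor objects.
; On activation it plays the ghost's connect montage; at the montage notify it fires the ghost's pulse and box-overlaps around the ghost.
; Found actors get ActivateMessage with a success gameplay cue; otherwise a fail cue plays.
; The ability ends after the notify, on montage completion or interruption, or if the avatar isn't a BP_HeroGhost.
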(event Ability|EventActivateAbility
  (bind _connectsize (Variables|Default|GetConnectSize))
  (bind _asbp_hero_ghost (Utilities|Casting|CastToBP_HeroGhost (Ability|GetAvatarActorfromActorInfo))
    (:then
      (Variables|Default|SetAs%20BP%20Hero%20Ghost _asbp_hero_ghost)
      (Animation|Montage|PlayMontage (Variables|/Script/Engine.Character|GetMesh (Variables|Default|GetAs%20BP%20Hero%20Ghost)) "/Game/Assets/Character/AceGhost/Animation/AM_AceGhost_Connect.AM_AceGhost_Connect"
        (:OnCompleted
          (Ability|EndAbility))
        (:OnInterrupted
          (Ability|EndAbility))
        (:OnNotifyBegin
          (Class|BPIHero|ActivatePulse(Message) (Variables|Default|GetAs%20BP%20Hero%20Ghost))
          (bind (_outactors _returnvalue) (Collision|BoxOverlapActors (Transformation|GetActorLocation (Variables|Default|GetAs%20BP%20Hero%20Ghost)) (Math|Vector|MakeVector _connectsize _connectsize _connectsize) (Utilities|Array|MakeArray "ObjectTypeQuery1" "ObjectTypeQuery2") "/Script/HeartWeaver.KrakenConnectableActor" :!class /Script/Engine.KismetSystemLibrary))
          (if _returnvalue
            (GameplayCue|ExecuteGameplayCue :GameplayCueTag "(TagName=\"GameplayCue.Character.Hero.Ability.Ability.Connect.Success\")")
            (for _array_element _outactors
              (Class|KrakenActivableObject|Activate(Message) _array_element))
            (else
              (GameplayCue|ExecuteGameplayCue :GameplayCueTag "(TagName=\"GameplayCue.Character.Hero.Ability.Ability.Connect.Fail\")")))
          (Ability|EndAbility))))
    (:CastFailed
      (Ability|EndAbility))))

(event Ability|EventOnEndAbility
  (params (bWasCancelled :type Boolean)))