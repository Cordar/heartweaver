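; GA_SendMark is a Hero gameplay ability that marks a target for the companion's AI.
; It resolves the companion's AI controller from the Hero, then runs a capsule trace forward from the companion's pawn, along that pawn's facing rather than the Hero's.
; A hit passes the impact location and actor to the controller's SetTargetActor.
; The ability ends immediately, whether or not anything is hit.
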(event Ability|EventOnEndAbility
  (params (bWasCancelled :type Boolean)))

(event Ability|EventActivateAbility
  (bind _asbp_hero (Utilities|Casting|CastToBP_Hero (Class|KrakenGameplayAbility|GetKrakenCharacterfromActorInfo))
    (:then
      (bind _asbp_companion_aicontroller (Utilities|Casting|CastToBP_CompanionAIController (AI|GetAIController (Variables|/Game/Blueprints/Character/Hero/BP_Hero.BP_Hero_C|GetBPCompanion _asbp_hero)))
        (:then
          (Variables|Default|SetAs%20BP%20Companion%20AIController _asbp_companion_aicontroller)
          (bind (_outhit _returnvalue) (Collision|CapsuleTraceByChannel (+ (* (Variables|Default|GetStartDistance) (Transformation|GetActorForwardVector (Pawn|GetControlledPawn (Variables|Default|GetAs%20BP%20Companion%20AIController)))) (Transformation|GetActorLocation (Pawn|GetControlledPawn (Variables|Default|GetAs%20BP%20Companion%20AIController)))) (+ (Transformation|GetActorLocation (Pawn|GetControlledPawn (Variables|Default|GetAs%20BP%20Companion%20AIController))) (* (Variables|Default|GetCheckDistance) (Transformation|GetActorForwardVector (Pawn|GetControlledPawn (Variables|Default|GetAs%20BP%20Companion%20AIController))))) (Variables|Default|GetCheckRadius) (Variables|Default|GetCheckHalfHeight) "TraceTypeQuery4" false 0 "None"))
          (if _returnvalue
            (Default|SetTargetActor (Variables|Default|GetAs%20BP%20Companion%20AIController) (.location _outhit) (.hitactor _outhit))
            (Ability|EndAbility)
            (else
              (Ability|EndAbility))))
        (:CastFailed
          (Ability|EndAbility))))
    (:CastFailed
      (Ability|EndAbility))))