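; GA_AimMark is a hero gameplay ability that puts the hero's companion into aim mode for marking.
; On activation it finds the companion's AI controller through the hero and activates aim on it, ending at once if either cast fails.
; It then waits for either input release or activation of a Send Mark ability, and either one deactivates the companion's aim and ends the ability.
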(event Ability|EventActivateAbility
  (bind _asbp_hero (Utilities|Casting|CastToBP_Hero (Class|KrakenGameplayAbility|GetKrakenCharacterfromActorInfo))
    (:then
      (bind _asbp_companion_aicontroller (Utilities|Casting|CastToBP_CompanionAIController (AI|GetAIController (Variables|/Game/Blueprints/Character/Hero/BP_Hero.BP_Hero_C|GetBPCompanion _asbp_hero)))
        (:then
          (bind _output_get (Variables|Default|SetAs%20BP%20Companion%20AIController _asbp_companion_aicontroller))
          (Default|ActivateAim _output_get)
          (|WaitforAbilityActivate :WithTag "(TagName=\"Ability.SendMark\")"
            (:then
              (Ability|Tasks|WaitInputRelease true
                (:OnRelease
                  _)))
            (:OnActivate
              _))
          (Default|DeactivateAim (Variables|Default|GetAs%20BP%20Companion%20AIController))
          (Ability|EndAbility))
        (:CastFailed
          (Ability|EndAbility))))
    (:CastFailed
      (Ability|EndAbility))))

(event Ability|EventOnEndAbility
  (params (bWasCancelled :type Boolean)))