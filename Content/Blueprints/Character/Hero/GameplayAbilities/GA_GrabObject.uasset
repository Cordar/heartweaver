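; Gameplay ability that toggles the hero grabbing and releasing a holdable object through KrakenPushComponent.
; If already holding, it ends the push; otherwise a short forward object trace sends HoldMessage to the hit actor.
; A successful grab adds loose gameplay tags and the IMC_GrabObject input context, which release removes.
; The ability ends immediately either way, and its interactable-actor helper functions are not called by the event graph.
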(event Ability|EventActivateAbility
  (bind _returnvalue (Class|KrakenGameplayAbility|GetKrakenCharacterfromActorInfo))
  (bind _returnvalue_2 (Class|KrakenGameplayAbility|GetKrakenCharacterfromActorInfo))
  (bind _returnvalue_3 (Class|KrakenGameplayAbility|GetKrakenCharacterfromActorInfo))
  (bind _returnvalue_4 (Actor|GetComponentbyClass _returnvalue_3 "/Script/HeartWeaver.KrakenPushComponent"))
  (bind _returnvalue_5 (Transformation|GetActorLocation _returnvalue))
  (if (Class|KrakenPushComponent|IsHoldingObject _returnvalue_4)
    (Class|KrakenPushComponent|EndPush _returnvalue_4)
    (Ability|GameplayEffect|RemoveLooseGameplayTags (Class|KrakenGameplayAbility|GetKrakenCharacterfromActorInfo) (Variables|Default|GetGameplayTagsAddedToActor))
    (Input|RemoveMappingContext (PlayerController|LocalPlayerSubsystems|GetEnhancedInputLocalPlayerSubsystem (Game|GetPlayerController 0)) "/Game/Blueprints/Input/IMC_GrabObject.IMC_GrabObject" "(bIgnoreAllPressedKeysUntilRelease=True,bForceImmediately=False,bNotifyUserSettings=False)")
    (Ability|EndAbility)
    (else
      (bind (_outhit _returnvalue_6) (Collision|LineTraceForObjects _returnvalue_5 (+ _returnvalue_5 (* (Transformation|GetActorForwardVector _returnvalue) 1e+02)) (Utilities|Array|MakeArray "ObjectTypeQuery7") false 0 "None"))
      (if _returnvalue_6
        (Class|KrakenPushableObject|Hold(Message) (.hitactor _outhit) _returnvalue_2)
        (if (Class|KrakenPushComponent|IsHoldingObject (Actor|GetComponentbyClass (Class|KrakenGameplayAbility|GetKrakenCharacterfromActorInfo) "/Script/HeartWeaver.KrakenPushComponent"))
          (Ability|GameplayEffect|AddLooseGameplayTags _returnvalue_2 (Variables|Default|GetGameplayTagsAddedToActor))
          (Input|AddMappingContext (PlayerController|LocalPlayerSubsystems|GetEnhancedInputLocalPlayerSubsystem (Game|GetPlayerController 0)) "/Game/Blueprints/Input/IMC_GrabObject.IMC_GrabObject" 1 "(bIgnoreAllPressedKeysUntilRelease=True,bForceImmediately=False,bNotifyUserSettings=False)"))
        (Ability|EndAbility)
        (else
          (Ability|EndAbility))))))

(event Ability|EventOnEndAbility
  (params (bWasCancelled :type Boolean)))

(fn FindInteractableActor
  (bind _returnvalue (Class|KrakenGameplayAbility|GetKrakenCharacterfromActorInfo))
  (bind _returnvalue_2 (Class|KrakenCharacter|GetInteractableActor _returnvalue))
  (Utilities|IsValid _returnvalue_2
    (:Is%20Valid
      (Variables|Default|SetOverlapped%20Interactable%20Actor _returnvalue_2)
      (return true))
    (:Is%20Not%20Valid
      (return false))))

(fn InteractwithActor
  (Class|KrakenActivableObject|Activate (Variables|Default|GetOverlapped%20Interactable%20Actor) (Class|KrakenGameplayAbility|GetKrakenCharacterfromActorInfo)))