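; Hero gameplay ability "Feel Sadness" that changes global time dilation for a limited time while its avatar keeps normal speed.
; On activation it applies a gameplay effect to the owner, then waits out a charge time before dilating time.
; The avatar's custom dilation is set to the inverse, and the feel delay is scaled by dilation to last in real seconds.
; Both dilations reset only when that delay finishes, as the end-ability event is empty.
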(event Ability|EventActivateAbility
  (Ability|ApplyGameplayEffectToOwner 0)
  (Ability|Tasks|WaitDelay (Variables|Default|GetChargeTime)
    (:OnFinish
      (Utilities|Time|SetGlobalTimeDilation (Variables|Default|GetTime%20Dilation))
      (Variables|/Script/Engine.Actor|SetCustomTimeDilation (Ability|GetAvatarActorfromActorInfo) (/ 1.0 (Variables|Default|GetTime%20Dilation)))
      (Ability|Tasks|WaitDelay (* (Variables|Default|GetFeelTime) (Variables|Default|GetTime%20Dilation))
        (:OnFinish
          (Utilities|Time|SetGlobalTimeDilation 1.0)
          (Variables|/Script/Engine.Actor|SetCustomTimeDilation (Ability|GetAvatarActorfromActorInfo) 1.0)
          (Ability|EndAbility))))))

(event Ability|EventOnEndAbility
  (params (bWasCancelled :type Boolean)))