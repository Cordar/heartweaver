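; BP_HeroGhost is a possessable ghost hero character that can glide to another pawn, possess it and destroy itself.
; It copies the player character's gravity on BeginPlay and binds to the GES gravity-switch event, with SwitchGravity inverting gravity Z.
; Possession makes BP_TrackingCamera follow it, retrying until one exists, and unpossession destroys it.
; The transfer uses flying mode, query-only collision and a timeline lerp tracking the target's live location.
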(event Custom|GoDirectlyToActorAndPossess
  (params (InPawn :type Pawn%20Object%20Reference))
  (Pawn|Components|CharacterMovement|SetMovementMode (Variables|Default|GetKrakenCharacterMovementComponent) "MOVE_Flying" 0)
  (Collision|SetCollisionEnabled (Variables|Default|GetCapsuleComponent) "QueryOnly")
  (Variables|Default|SetLocationBeforeTP (Transformation|GetActorLocation))
  (bind _distance (Timeline|MoveToActor Play)
    (:Update
      (Transformation|SetActorLocation (Math|Vector|Lerp(Vector) (Variables|Default|GetLocationBeforeTP) (Transformation|GetActorLocation InPawn) _distance) false true))
    (:Finished
      (Pawn|Possess (Game|GetPlayerController 0) InPawn)
      (Actor|DestroyActor))))

(event EventBeginPlay
  (bind _askraken_character (Utilities|Casting|CastToKrakenCharacter (Game|GetPlayerCharacter 0)))
  (Class|CharacterMovementComponent|SetGravityDirection (Variables|Default|GetKrakenCharacterMovementComponent) (Class|CharacterMovementComponent|GetGravityDirection (Variables|/Script/HeartWeaver.KrakenCharacter|GetKrakenCharacterMovementComponent _askraken_character)))
  (Class|GlobalEventSystemBPLibrary|GESBindTagEventtoDelegate "(TagName=\"Event.Gravity.Switch\")" (EventDispatchers|CreateEvent :!event SwitchGravity)))

(event EventUnpossessed
  (params (OldController :type Controller%20Object%20Reference))
  (Actor|DestroyActor))

(event EventPossessed
  (params (NewController :type Controller%20Object%20Reference))
  (CallFunction|ActivateCamera))

(event EventEndPlay
  (params (EndPlayReason :type EEndPlayReason%20Enum :default "Destroyed"))
  (Class|GlobalEventSystemBPLibrary|GESUnbindTagDelegate "(TagName=\"Event.Gravity.Switch\")" (EventDispatchers|CreateEvent :!event SwitchGravity)))

(fn ConstructionScript
  (Class|KrakenCharacter|SetLayingonFloor false))

(fn ActivateCamera
  (bind _returnvalue (Actor|GetActorOfClass "/Game/Blueprints/Camera/BP_TrackingCamera.BP_TrackingCamera_C"))
  (Utilities|IsValid _returnvalue
    (:Is%20Valid
      (Variables|/Game/Blueprints/Camera/BP_TrackingCamera.BP_TrackingCamera_C|SetCharacterToFollow _returnvalue self)
      (Variables|Default|SetFollowCamera _returnvalue))
    (:Is%20Not%20Valid
      (Utilities|Time|SetTimerbyFunctionName 0 "ActivateCamera" 0.1))))

(fn SwitchGravity
  (params (WildcardProperty :type GES%20Wildcard%20Property%20Structure%20%28by%20ref%29))
  (bind _krakencharactermovementcomponent (Variables|Default|GetKrakenCharacterMovementComponent))
  (bind _gravitydirection (Variables|/Script/Engine.CharacterMovementComponent|GetGravityDirection _krakencharactermovementcomponent))
  (Class|KrakenCharacterMovementComponent|ChangeGravityDirection _krakencharactermovementcomponent (Math|Vector|MakeVector (.x _gravitydirection) (.y _gravitydirection) (* (.z _gravitydirection) -1.0)))
  (return))