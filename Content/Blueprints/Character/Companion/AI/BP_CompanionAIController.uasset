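; AI controller for the hero's companion, running the BT_Mark behavior tree with the hero as its PlayerActor.
; Each tick it reads the blackboard State: idle and near-player states turn it toward the hero, and idle also pushes it out of a minimum radius.
; Aiming shows the cursor and snaps the companion around the hero toward the mouse ray's intersection with the hero's plane.
; Rotation and avoidance work in hero space, respecting the hero's up vector.
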(event Custom|ActivateAim
  ;[0.6749 0.7151 0.8438] Aim
  (Variables|/Script/Engine.PlayerController|SetbShowMouseCursor (Game|GetPlayerController 0) true)
  (AI|Components|Blackboard|SetValueasEnum (Variables|Default|GetBlackboard) (Utilities|Name|MakeLiteralName "State") (Utilities|Enum|LiteralenumEMarkAction "NewEnumerator2"))
  (AI|Navigation|StopMovement))

(event Custom|DeactivateAim
  ;[0.6749 0.7151 0.8438] Aim
  (Variables|/Script/Engine.PlayerController|SetbShowMouseCursor (Game|GetPlayerController 0) false)
  (AI|Components|Blackboard|SetValueasEnum (Variables|Default|GetBlackboard) (Utilities|Name|MakeLiteralName "State") (Utilities|Enum|LiteralenumEMarkAction "NewEnumerator0")))

(event Custom|AimMark
  (bind _returnvalue (Game|GetPlayerController 0))
  (bind _returnvalue_2 (Pawn|GetControlledPawn))
  (bind _returnvalue_3 (Math|Float|MakeLiteralFloat 9999999.0))
  (bind _hero (Variables|Default|GetHero))
  (bind _hero_2 (Variables|Default|GetHero))
  (bind _hero_3 (Variables|Default|GetHero))
  (bind _returnvalue_4 (Transformation|GetActorLocation _hero_2))
  (bind (_locationx _locationy) (Game|Player|GetMousePosition _returnvalue))
  (bind _returnvalue_5 (Transformation|GetActorUpVector _hero_2))
  (bind _returnvalue_6 (Transformation|GetActorLocation _hero))
  (bind _returnvalue_7 (Transformation|GetActorTransform _hero_3))
  (bind (_worldlocation _worlddirection) (Class|PlayerController|DeprojectScreenPositiontoWorld _returnvalue _locationx _locationy))
  (bind _returnvalue_8 (* _worlddirection _returnvalue_3))
  (bind _returnvalue_9 (+ _worldlocation _returnvalue_8))
  (bind _intersection (Class|KismetMathLibrary|LinePlaneIntersectionOriginNormal _worldlocation _returnvalue_9 _returnvalue_4 _returnvalue_5))
  ;[0.6749 0.7151 0.8438] Aim Mark
  (Transformation|SetActorLocation _returnvalue_2 (+ _returnvalue_6 (* (Math|Vector|Normalize (- _intersection _returnvalue_6)) (Math|Float|MakeLiteralFloat 1.3e+02))) false true)
  (Transformation|SetActorRotation _returnvalue_2 (Math|Transform|TransformRotation _returnvalue_7 (Math|Rotator|FindLookatRotation (Math|Vector|MakeVector 0.0 0.0 0.0) (Math|Transform|InverseTransformLocation _returnvalue_7 _intersection)))))

(event Custom|LookAtPlayer
  (params (Delta :type Float%20%28double-precision%29))
  ;[1 1 1] Look at player
  (CallFunction|LookatActor (Variables|Default|GetHero) (* Delta 4.0)))

(event Custom|AvoidPlayer
  (bind _returnvalue (Pawn|GetControlledPawn))
  (bind _returnvalue_2 (Pawn|GetControlledPawn))
  (bind _returnvalue_3 (AI|GetBlackboard 0))
  (bind _returnvalue_4 (Utilities|Name|MakeLiteralName "MinIdleRadius"))
  (bind _hero (Variables|Default|GetHero))
  (bind _returnvalue_5 (Pawn|GetMovementComponent _returnvalue))
  (bind _returnvalue_6 (Transformation|GetActorTransform _hero))
  (bind _returnvalue_7 (Transformation|GetActorLocation _returnvalue_2))
  (bind _returnvalue_8 (Class|BlackboardComponent|GetValueasFloat _returnvalue_3 _returnvalue_4))
  (bind _returnvalue_9 (Math|Transform|InverseTransformLocation _returnvalue_6 _returnvalue_7))
  (bind _returnvalue_10 (Math|Vector|MakeVector (.x _returnvalue_9) (.y _returnvalue_9) 0.0))
  (bind _returnvalue_11 (Math|Vector|VectorLength _returnvalue_10))
  ;[1 0.9242 0.9443] Avoid Player
  (if (not (<= _returnvalue_11 1e+01))
    (if (< _returnvalue_11 _returnvalue_8)
      (Variables|/Script/Engine.MovementComponent|SetVelocity _returnvalue_5 (Math|Transform|TransformDirection (Transformation|GetActorTransform (Variables|Default|GetHero)) (* (Math|Vector|Normalize _returnvalue_10) (Math|Float|MakeLiteralFloat 5e+01) (/ _returnvalue_8 _returnvalue_11))))
      (else
        (Variables|/Script/Engine.MovementComponent|SetVelocity _returnvalue_5 (* (Variables|/Script/Engine.MovementComponent|GetVelocity _returnvalue_5) (Math|Float|MakeLiteralFloat 0.9)))))))

(event Custom|DrawDebugRadious
  (bind _returnvalue (Pawn|GetControlledPawn))
  (bind _returnvalue_2 (Utilities|Name|MakeLiteralName "MaxIdleRadius"))
  (bind _returnvalue_3 (Utilities|Name|MakeLiteralName "MinIdleRadius"))
  (bind _returnvalue_4 (AI|GetBlackboard _returnvalue))
  (bind _returnvalue_5 (Class|BlackboardComponent|GetValueasFloat _returnvalue_4 _returnvalue_2))
  (bind _returnvalue_6 (Class|BlackboardComponent|GetValueasFloat _returnvalue_4 _returnvalue_3))
  (bind _hero (Variables|Default|GetHero)
    (:then
      (Rendering|Debug|DrawDebugCircle (Transformation|GetActorLocation _hero) _returnvalue_6 20 "(R=1.000000,G=0.000000,B=0.078214,A=1.000000)" 0.0 0.0 "1.000000,0.000000,0.000000" "0.000000,1.000000,0.000000")
      (Rendering|Debug|DrawDebugCircle (Transformation|GetActorLocation _hero) _returnvalue_5 20 "(R=0.939690,G=1.000000,B=0.000000,A=1.000000)" 0.0 0.0 "1.000000,0.000000,0.000000" "0.000000,1.000000,0.000000")
      (Rendering|Debug|DrawDebugCircle (Transformation|GetActorLocation _hero) (/ (+ _returnvalue_6 _returnvalue_5) 2.0) 20 "(R=0.000000,G=1.000000,B=0.323878,A=1.000000)" 0.0 0.0 "1.000000,0.000000,0.000000" "0.000000,1.000000,0.000000"))
    (:else)))

(event EventBeginPlay
  ;[1 1 1] Beginplay
  (bind _asbp_hero (Utilities|Casting|CastToBP_Hero (Game|GetPlayerCharacter 0)))
  (Variables|Default|SetHero _asbp_hero))

(event EventTick
  (params (DeltaSeconds :type Float%20%28single-precision%29))
  ;[0.6749 0.7151 0.8438] Event Tick
  (Utilities|FlowControl|Sequence
    (:then_0
      (switch Utilities|FlowControl|Switch|SwitchonEMarkAction (Utilities|Enum|ByteToEnumEMarkAction (Class|BlackboardComponent|GetValueasEnum (Variables|Default|GetBlackboard) (Utilities|Name|MakeLiteralName "State")))
        (:NewEnumerator0
          (CallFunction|LookatPlayer DeltaSeconds)
          (CallFunction|AvoidPlayer))
        (:NewEnumerator1
          (CallFunction|LookatPlayer DeltaSeconds))
        (:NewEnumerator2
          (CallFunction|AimMark))))))

(event EventPossess
  (params (PossessedPawn :type Pawn%20Object%20Reference))
  ;[0.6749 0.7151 0.8438] On Posses
  (AI|RunBehaviorTree "/Game/Blueprints/Character/Companion/AI/Mark/BT_Mark.BT_Mark")
  (AI|Components|Blackboard|SetValueasObject (Variables|Default|GetBlackboard) (Utilities|String|StringToName "PlayerActor") (Variables|Default|GetHero)))

(fn ConstructionScript)

(fn GetIAState
  (return (Utilities|Enum|ByteToEnumEMarkAction (Class|BlackboardComponent|GetValueasEnum (AI|GetBlackboard (Pawn|GetControlledPawn)) (Utilities|Name|MakeLiteralName "State")))))

(fn SetIAState
  (params (NewState :type EMarkAction%20Enum :default "NewEnumerator0"))
  (AI|Components|Blackboard|SetValueasEnum (AI|GetBlackboard (Pawn|GetControlledPawn)) (Utilities|Name|MakeLiteralName "State") NewState))

(fn SetAITargetActor
  (params (Target :type Actor%20Object%20Reference))
  (AI|Components|Blackboard|SetValueasObject (AI|GetBlackboard (Pawn|GetControlledPawn)) (Utilities|Name|MakeLiteralName "TargetActor") Target))

(fn GetAITargetActor
  (return (.AsActor (Utilities|Casting|CastToActor (AI|Components|Blackboard|GetValueasObject (AI|GetBlackboard (Pawn|GetControlledPawn)) (Utilities|Name|MakeLiteralName "TargetActor"))))))

(fn LookatActor
  (params (ActorTarget :type Actor%20Object%20Reference) (Alpha :type Float%20%28double-precision%29))
  (bind _returnvalue (Pawn|GetControlledPawn))
  (bind _returnvalue_2 (Transformation|GetActorTransform ActorTarget))
  (Transformation|SetActorRotation _returnvalue (Math|Rotator|Lerp(Rotator) (Transformation|GetActorRotation _returnvalue) (Math|Transform|TransformRotation _returnvalue_2 (Math|Rotator|FindLookatRotation (Math|Vector|MakeVector 0.0 0.0 0.0) (Math|Vector|NegateVector (Math|Transform|InverseTransformLocation _returnvalue_2 (Transformation|GetActorLocation _returnvalue))))) Alpha true)))

(fn GetClosestPointatPlayerCircle
  (params (Radius :type Float%20%28double-precision%29))
  (bind _returnvalue (Pawn|GetControlledPawn))
  (bind _hero (Variables|Default|GetHero))
  (bind _hero_2 (Variables|Default|GetHero))
  (bind _returnvalue_2 (Transformation|GetActorTransform _hero))
  (bind _returnvalue_3 (Transformation|GetActorLocation _hero_2))
  (bind _returnvalue_4 (Transformation|GetActorLocation _returnvalue))
  (bind _returnvalue_5 (- _returnvalue_4 _returnvalue_3))
  (bind _returnvalue_6 (Math|Vector|Normalize _returnvalue_5))
  (bind _returnvalue_7 (Math|Transform|InverseTransformDirection _returnvalue_2 _returnvalue_6))
  (bind (_x _y) (Math|Vector|BreakVector _returnvalue_7))
  (return (+ (Transformation|GetActorLocation _hero) (* (Math|Transform|TransformDirection _returnvalue_2 (Math|Vector|Normalize (Math|Vector|MakeVector _x _y 0.0))) Radius))))