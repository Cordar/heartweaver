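; BPF_Save is a Blueprint function library for quick-saving and loading the player's location through a BP_SaveGame object.
; SaveGame creates a new save object each call, stores the given PlayerLocation, writes it synchronously to the fixed "QuickSave" slot and returns it.
; LoadGame reads the same slot, checks validity, and returns a Found flag with the cast save object, leaving applying the location to the caller.
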(fn SaveGame
  (params (PlayerLocation :type Vector))
  (bind _returnvalue (SaveGame|CreateSaveGameObject "/Game/Blueprints/Game/BP_SaveGame.BP_SaveGame_C"))
  (bind _output_get (LocalVariables|SetSaveGameObject _returnvalue))
  (Variables|/Game/Blueprints/Game/BP_SaveGame.BP_SaveGame_C|SetPlayerLocation (LocalVariables|GetSaveGameObject) PlayerLocation)
  (SaveGame|SaveGametoSlot (LocalVariables|GetSaveGameObject) "QuickSave")
  (return _output_get))

(fn LoadGame
  (bind _returnvalue (SaveGame|LoadGamefromSlot "QuickSave"))
  (Utilities|IsValid _returnvalue
    (:Is%20Valid
      (bind _asbp_save_game (Utilities|Casting|CastToBP_SaveGame _returnvalue))
      (return true _asbp_save_game))
    (:Is%20Not%20Valid
      (return false 0))))