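; Test VFX actor that builds a radial cluster of Niagara tentacles.
; The construction script loops up to NumberOfTentacles, adding three Niagara components per index, each rotated on a different pair of axes by index times Distance.
; Odd indices negate the angles, and every component receives the same NiagaraSystem.
; BeginPlay only zeroes OriginLocation; Tick is empty, and the player-chasing interpolation is disconnected, so it never runs.
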(event EventTick
  (params (DeltaSeconds :type Float%20%28single-precision%29)))

(event EventBeginPlay
  (Variables|Default|SetOriginLocation "0, 0, 0"))

(fn ConstructionScript
  (for _index (range 0 (Variables|Default|GetNumberOfTentacles))
    (if (== (Math|Integer|%(Integer) _index 2) 0)
      (bind _returnvalue (AddComponent|AddNiagaraComponent false (Math|Transform|MakeTransform "0, 0, 0" (Math|Rotator|MakeRotator 0.0 (* (Math|Conversions|ToFloat(Integer) _index) (Variables|Default|GetDistance)) (* (Math|Conversions|ToFloat(Integer) _index) (Variables|Default|GetDistance))) "1.000000,1.000000,1.000000")))
      (Class|NiagaraComponent|SetAsset _returnvalue (Variables|Default|GetNiagaraSystem) true)
      (bind _returnvalue_2 (AddComponent|AddNiagaraComponent false (Math|Transform|MakeTransform "0, 0, 0" (Math|Rotator|MakeRotator (* (Math|Conversions|ToFloat(Integer) _index) (Variables|Default|GetDistance)) (* (Math|Conversions|ToFloat(Integer) _index) (Variables|Default|GetDistance)) 0.0) "1.000000,1.000000,1.000000")))
      (Class|NiagaraComponent|SetAsset _returnvalue_2 (Variables|Default|GetNiagaraSystem) true)
      (bind _returnvalue_3 (AddComponent|AddNiagaraComponent false (Math|Transform|MakeTransform "0, 0, 0" (Math|Rotator|MakeRotator (* (Math|Conversions|ToFloat(Integer) _index) (Variables|Default|GetDistance)) 0.0 (* (Math|Conversions|ToFloat(Integer) _index) (Variables|Default|GetDistance))) "1.000000,1.000000,1.000000")))
      (Class|NiagaraComponent|SetAsset _returnvalue_3 (Variables|Default|GetNiagaraSystem) true)
      (else
        (bind _returnvalue_4 (AddComponent|AddNiagaraComponent false (Math|Transform|MakeTransform "0, 0, 0" (Math|Rotator|MakeRotator 0.0 (* (Math|Conversions|ToFloat(Integer) _index) (Variables|Default|GetDistance) -1.0) (* (Math|Conversions|ToFloat(Integer) _index) (Variables|Default|GetDistance) -1.0)) "1.000000,1.000000,1.000000")))
        (Class|NiagaraComponent|SetAsset _returnvalue_4 (Variables|Default|GetNiagaraSystem) true)
        (bind _returnvalue_5 (AddComponent|AddNiagaraComponent false (Math|Transform|MakeTransform (Math|Vector|MakeVector 0.0 0.0 0.0) (Math|Rotator|MakeRotator (* (Math|Conversions|ToFloat(Integer) _index) (Variables|Default|GetDistance) -1.0) (* (Math|Conversions|ToFloat(Integer) _index) (Variables|Default|GetDistance) -1.0) 0.0) "1.000000,1.000000,1.000000")))
        (Class|NiagaraComponent|SetAsset _returnvalue_5 (Variables|Default|GetNiagaraSystem) true)
        (bind _returnvalue_6 (AddComponent|AddNiagaraComponent false (Math|Transform|MakeTransform "0, 0, 0" (Math|Rotator|MakeRotator (* (Math|Conversions|ToFloat(Integer) _index) (Variables|Default|GetDistance) -1.0) 0.0 (* (Math|Conversions|ToFloat(Integer) _index) (Variables|Default|GetDistance) -1.0)) "1.000000,1.000000,1.000000")))
        (Class|NiagaraComponent|SetAsset _returnvalue_6 (Variables|Default|GetNiagaraSystem) true)))))