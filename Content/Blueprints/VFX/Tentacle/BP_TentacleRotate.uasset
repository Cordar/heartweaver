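; BP_TentacleRotate is a tentacle VFX actor that removes itself when its linked puzzle is solved.
; On BeginPlay it caches BP_GameInstance, queries it for the puzzle's solved state and calls Disappear if solved.
; Disappear uses a timeline to move the actor vertically by DeathHeight from its starting Z, then destroys it.
; Despite the name, its graphs contain no rotation logic.
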(event Custom|Disappear
  (bind _returnvalue (Transformation|GetActorLocation))
  (bind _move (Timeline|Timeline PlayFromStart)
    (:Update
      (Transformation|SetActorLocation (Math|Vector|MakeVector (.x _returnvalue) (.y _returnvalue) (Math|Float|Lerp (Variables|Default|GetOriginalHeight) (+ (Variables|Default|GetOriginalHeight) (Variables|Default|GetDeathHeight)) _move)) false false))
    (:Finished
      (Actor|DestroyActor))))

(event EventBeginPlay
  (CallFunction|GetGameInstance)
  (CallFunction|DisappearifPuzzleCompleted)
  (Variables|Default|SetOriginalHeight (.z (Transformation|GetActorLocation))))

(fn ConstructionScript)

(fn BPTentacleRotateAutoGenFunc)

(fn DisappearifPuzzleCompleted
  (bind _issolved (Default|IsPuzzleSolved (Variables|Default|GetAs%20BP%20Game%20Instance) (Variables|Default|GetPuzzle)))
  (if _issolved
    (CallFunction|Disappear)))

(fn GetGameInstance
  (bind _asbp_game_instance (Utilities|Casting|CastToBP_GameInstance (Game|GetGameInstance)))
  (Variables|Default|SetAs%20BP%20Game%20Instance _asbp_game_instance))