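; BP_TentacleRotate_Brilli_dark_Wigle1 is a tentacle VFX actor that can move out of the level vertically and remove itself.
; On BeginPlay it stores its starting height and, if a PuzzleEntrance reference is valid, binds to that entrance's puzzle-solved event, presumably to trigger Disappear.
; Disappear plays a timeline that lerps the actor's Z by DeathHeight from the stored height, then destroys the actor.
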(event Custom|Disappear
  (bind _returnvalue (Transformation|GetActorLocation))
  (bind _move (Timeline|Timeline PlayFromStart)
    (:Update
      (Transformation|SetActorLocation (Math|Vector|MakeVector (.x _returnvalue) (.y _returnvalue) (Math|Float|Lerp (Variables|Default|GetOriginalHeight) (+ (Variables|Default|GetOriginalHeight) (Variables|Default|GetDeathHeight)) _move)) false false))
    (:Finished
      (Actor|DestroyActor))))

(event EventBeginPlay
  (bind _puzzleentrance (Variables|Default|GetPuzzleEntrance))
  (Variables|Default|SetOriginalHeight (.z (Transformation|GetActorLocation)))
  (Utilities|IsValid _puzzleentrance
    (:Is%20Valid
      (EventDispatchers|BindEventtoOnPuzzleSolved _puzzleentrance (EventDispatchers|CreateEvent :!event Custom|Disappear)))))

(fn ConstructionScript)

(fn BPTentacleRotateAutoGenFunc)