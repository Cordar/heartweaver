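; BP_TentacleRotate_Brilli_Wigle is a tentacle actor that can move vertically out of place and destroy itself, apparently when a puzzle is solved.
; On BeginPlay it binds to PuzzleEntrance's OnPuzzleSolved and stores its starting Z.
; Disappear plays a timeline that lerps Z from that height by a DeathHeight offset, then destroys the actor.
; The construction script and auto-generated function are empty.
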(event Custom|Disappear
  (bind _returnvalue (Transformation|GetActorLocation))
  (bind _move (Timeline|Timeline PlayFromStart)
    (:Update
      (Transformation|SetActorLocation (Math|Vector|MakeVector (.x _returnvalue) (.y _returnvalue) (Math|Float|Lerp (Variables|Default|GetOriginalHeight) (+ (Variables|Default|GetOriginalHeight) (Variables|Default|GetDeathHeight)) _move)) false false))
    (:Finished
      (Actor|DestroyActor))))

(event EventBeginPlay
  (EventDispatchers|BindEventtoOnPuzzleSolved (Variables|Default|GetPuzzleEntrance) (EventDispatchers|CreateEvent :!event Custom|Disappear))
  (Variables|Default|SetOriginalHeight (.z (Transformation|GetActorLocation))))

(fn ConstructionScript)

(fn BPTentacleRotateAutoGenFunc)