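; Tracking camera that smoothly turns toward the followed character, or an optional look target, using lag-scaled lerps.
; BP_TriggerCamera actors set its location and spline at start; BeginPlay also overrides lag values for the "numbness" level.
; Each tick it eases toward a target location or the spline point nearest the character, snapping when far away.
; It also overrides the audio listener, combining character XY, interpolated height and camera-based rotation.
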(event Custom|LookToPlayer
  (params (Delta :type Float%20%28double-precision%29) (Power :type Float%20%28double-precision%29))
  (Transformation|SetActorRotation (Math|Rotator|Lerp(Rotator) (Transformation|GetActorRotation) (CallFunction|GetTargetRotation) (* Delta Power) true) true))

(event Custom|MoveToTarget
  (params (Delta :type Float%20%28double-precision%29) (Power :type Float%20%28double-precision%29))
  (Transformation|SetActorLocation (Math|Vector|Lerp(Vector) (Transformation|GetActorLocation) (Variables|Default|GetTargetLocation) (* Delta Power)) false true))

(event Custom|MoveAudioListener
  (params (Delta :type Float%20%28double-precision%29) (Power :type Float%20%28double-precision%29))
  (bind _charactertofollow (Variables|Default|GetCharacterToFollow))
  (bind _mesh (Variables|/Script/Engine.Character|GetMesh _charactertofollow))
  (bind _returnvalue (Transformation|GetWorldLocation _mesh))
  (Class|PlayerController|SetAudioListenerOverride (Game|GetPlayerController 0) 0 (Math|Vector|MakeVector (.x _returnvalue) (.y _returnvalue) (.z (Math|Vector|Lerp(Vector) (Variables|Default|GetAudioListenerLocation) (Variables|Default|GetAudioListenerTargetLocation) (* Delta Power)))) (Math|Rotator|Lerp(Rotator) (Transformation|GetActorRotation) (CallFunction|GetTargetRotation) (* Delta Power) true)))

(event Custom|FollowSpline
  (bind _scenecomponent (Variables|Default|GetSceneComponent))
  (bind _scenecomponent_2 (Variables|Default|GetSceneComponent))
  (bind _splinetofollow (Variables|Default|GetSplineToFollow))
  (bind _charactertofollow (Variables|Default|GetCharacterToFollow))
  (bind _returnvalue (Transformation|GetActorLocation _charactertofollow))
  (bind _returnvalue_2 (Transformation|GetWorldLocation _scenecomponent))
  (bind _returnvalue_3 (Spline|FindLocationClosesttoWorldLocation _splinetofollow _returnvalue "World"))
  (if (>= (Math|Vector|Distance(Vector) _returnvalue_2 _returnvalue_3) 2e+03)
    (Transformation|SetWorldLocation _scenecomponent_2 _returnvalue_3 false false)
    (Transformation|SetActorRotation (Math|Rotator|FindLookatRotation _returnvalue_3 (Transformation|GetActorLocation (Game|GetPlayerCharacter 0))))
    (else
      (Transformation|SetWorldLocation _scenecomponent_2 (Math|Interpolation|VInterpTo _returnvalue_2 _returnvalue_3 (Utilities|Time|GetWorldDeltaSeconds) (Variables|Default|GetMoveLag)) false false))))

(event EventBeginPlay
  (bind _returnvalue (Game|GetPlayerCharacter 0))
  (bind _initialtrigger (Variables|Default|GetInitialTrigger))
  (bind _overlappingactors (Collision|GetOverlappingActors _returnvalue "/Game/Blueprints/Camera/BP_TriggerCamera.BP_TriggerCamera_C" :!class /Script/Engine.Actor))
  (bind _returnvalue_2 (Game|GetCurrentLevelName true))
  (if (Utilities|Enum|Equal(Enum) _returnvalue_2 "numbness")
    (Variables|Default|SetRotationLag 1.0)
    (Variables|Default|SetMoveLag 2.0))
  (Utilities|IsValid _initialtrigger
    (:Is%20Valid
      (Default|SetCameraLocationandSpline _initialtrigger self))
    (:Is%20Not%20Valid
      _))
  (if (Utilities|Array|IsNotEmpty _overlappingactors)
    (bind _asbp_trigger_camera (Utilities|Casting|CastToBP_TriggerCamera (Utilities|Array|Get(acopy) _overlappingactors)))
    (Default|SetCameraLocationandSpline _asbp_trigger_camera self)
    (else
      (Variables|Default|SetTargetLocation (Transformation|GetActorLocation)))))

(event EventTick
  (params (DeltaSeconds :type Float%20%28single-precision%29))
  (bind _movelag (Variables|Default|GetMoveLag))
  (CallFunction|LooktoPlayer DeltaSeconds (Variables|Default|GetRotationLag))
  (Utilities|IsValid (Variables|Default|GetSplineToFollow)
    (:Is%20Valid
      (CallFunction|FollowSpline))
    (:Is%20Not%20Valid
      (CallFunction|MovetoTarget DeltaSeconds _movelag)))
  (CallFunction|MoveAudioListener DeltaSeconds _movelag))

(fn ConstructionScript)

(fn GetTargetRotation
  (bind _returnvalue (Transformation|GetActorLocation))
  (bind _looktarget (Variables|Default|GetLookTarget))
  (Utilities|IsValid _looktarget
    (:Is%20Valid
      (return (Math|Rotator|FindLookatRotation _returnvalue (Transformation|GetActorLocation _looktarget))))
    (:Is%20Not%20Valid
      (return (Math|Rotator|FindLookatRotation _returnvalue (Transformation|GetActorLocation (Variables|Default|GetCharacterToFollow)))))))