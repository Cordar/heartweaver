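; Game mode for HeartWeaver that handles game over and level restarts.
; GameOver records the current level name, calls Die on the player's BP_Hero, starts a three-second timer and immediately shows a loading widget.
; A separate OpenLevel event, apparently the timer's callback, reopens that same level by name.
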(event Custom|GameOver
  (bind _returnvalue (Game|GetCurrentLevelName true))
  (Variables|Default|SetLevelToOpen (Utilities|String|StringToName _returnvalue))
  (bind _asbp_hero (Utilities|Casting|CastToBP_Hero (Game|GetPlayerCharacter 0)))
  (Default|Die _asbp_hero)
  (Utilities|Time|SetTimerbyEvent (EventDispatchers|CreateEvent :!event Custom|OpenLevel) 3.0)
  (bind _returnvalue_2 (UserInterface|CreateWidget "/Game/Blueprints/UI/Widget/LoadingScreen/BPW_Loading.BPW_Loading_C" (Game|GetPlayerController 0)))
  (UserInterface|Viewport|AddtoViewport _returnvalue_2 0))

(event Custom|OpenLevel
  (Game|OpenLevel(byName) (Utilities|String|StringToName (stale Custom|GameOver _returnvalue))))

(fn ConstructionScript)