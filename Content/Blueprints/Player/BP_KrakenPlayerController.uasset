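; Player controller for the Kraken game that handles opening and closing the pause menu.
; Escape or P creates a WPB_PauseMenu widget, adds it to the viewport, pauses the game, shows the cursor and switches to Game and UI input focused on the menu.
; The ResumeGame event removes the stored widget, hides the cursor, restores game-only input and unpauses.
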(event Custom|ResumeGame
  (Widget|RemovefromParent (Variables|Default|GetPauseMenuWidget))
  (Variables|/Script/Engine.PlayerController|SetbShowMouseCursor self false)
  (Input|SetInputModeGameOnly self false)
  (Game|SetGamePaused false))

(event EventBeginPlay)

(event EventTick
  (params (DeltaSeconds :type Float%20%28single-precision%29)))

(event Input|KeyboardEvents|Escape
  (params (Key :type Key%20Structure))
  (:Pressed
    (bind _returnvalue (UserInterface|CreateWidget "/Game/Blueprints/UI/Widget/PauseMenu/WPB_PauseMenu.WPB_PauseMenu_C" (Game|GetPlayerController 0)))
    (Variables|Default|SetPauseMenuWidget _returnvalue)
    (UserInterface|Viewport|AddtoViewport (Variables|Default|GetPauseMenuWidget) 0)
    (Game|SetGamePaused true)
    (Variables|Default|SetbShowMouseCursor true)
    (Input|SetInputModeGameandUI self (Variables|Default|GetPauseMenuWidget) "DoNotLock" true false)))

(event Input|KeyboardEvents|P
  (params (Key :type Key%20Structure))
  (:Pressed
    (bind _returnvalue (UserInterface|CreateWidget "/Game/Blueprints/UI/Widget/PauseMenu/WPB_PauseMenu.WPB_PauseMenu_C" (Game|GetPlayerController 0)))
    (Variables|Default|SetPauseMenuWidget _returnvalue)
    (UserInterface|Viewport|AddtoViewport (Variables|Default|GetPauseMenuWidget) 0)
    (Game|SetGamePaused true)
    (Variables|Default|SetbShowMouseCursor true)
    (Input|SetInputModeGameandUI self (Variables|Default|GetPauseMenuWidget) "DoNotLock" true false)))

(fn ConstructionScript)